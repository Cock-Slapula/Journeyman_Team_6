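; BarrelLeft_BP is a rolling barrel hazard that launches its physics Cylinder along +Y on BeginPlay.
; It constrains the Cylinder to the YZ plane and applies a one-time velocity-change impulse.
; A looping one-second Delay reapplies the constraint and a timed boost, which is currently zero.
; The Box overlap event is empty, and the logic to destroy Mario_Character is disconnected, so the barrel does not kill the player.
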(event OnComponentBeginOverlap(Box)
  (params (OverlappedComponent :type Primitive%20Component%20Object%20Reference) (OtherActor :type Actor%20Object%20Reference) (OtherComp :type Primitive%20Component%20Object%20Reference) (OtherBodyIndex :type Integer) (bFromSweep :type Boolean) (SweepResult :type Hit%20Result%20Structure%20%28by%20ref%29))
  ;[1 1 1] Kill player if they hit the barrel
)

(event EventBeginPlay
  (bind _cylinder (Variables|Default|GetCylinder))
  (bind _cylinder_2 (Variables|Default|GetCylinder))
  (Utilities|FlowControl|Sequence
    (:then_0
      ;[1 1 1] Initial boost
      (Class|PrimitiveComponent|SetConstraintMode _cylinder "YZPlane")
      (bind _output_get (Variables|Default|SetInitial_Boost "0,550.000000, 0"))
      (Physics|AddImpulse _cylinder _output_get "None" true))
    (:then_1
      ;[1 1 1] Added boost
      (Utilities|FlowControl|Delay 1.0 :!label _label)
      (Class|PrimitiveComponent|SetConstraintMode _cylinder_2 "YZPlane")
      (bind _output_get_2 (Variables|Default|SetTimedBoost "0, 0, 0"))
      (Physics|AddImpulse _cylinder_2 _output_get_2 "None" true)
      (goto _label))))

(fn ConstructionScript)