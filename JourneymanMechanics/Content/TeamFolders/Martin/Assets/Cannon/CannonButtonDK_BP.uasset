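; Pressure-plate cannon button that spawns a Cannon_BP at its BarrelSpawnPoint on BeginPlay and fires it when Mario_Character steps on the plate.
; The overlap passes a DoOnce with no reset, so it triggers once, flashing two Cube material slots green before returning them to red.
; It also spawns a CannonBallDK_BP at the BarrelArrow of the first Cannon_BP found in the level, not necessarily its own.
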(event OnComponentBeginOverlap(PressurePlate)
  (params (OverlappedComponent :type Primitive%20Component%20Object%20Reference) (OtherActor :type Actor%20Object%20Reference) (OtherComp :type Primitive%20Component%20Object%20Reference) (OtherBodyIndex :type Integer) (bFromSweep :type Boolean) (SweepResult :type Hit%20Result%20Structure%20%28by%20ref%29))
  (bind _cube (Variables|Default|GetCube))
  (bind _cube_2 (Variables|Default|GetCube))
  ;[1 1 1] Change colour of pressure plate, cannon wire and cannon ring, revert back to red after .2 seconds
  (Utilities|Casting|CastToMario_Character OtherActor)
  (Utilities|FlowControl|DoOnce false
    (:Completed
      (Utilities|FlowControl|Sequence
        (:then_0
          (Rendering|Material|SetMaterial _cube 0 "/Game/TeamFolders/Martin/Materials/M_Green_Glow.M_Green_Glow")
          (Rendering|Material|SetMaterial _cube 2 "/Game/TeamFolders/Martin/Materials/M_Green_Glow.M_Green_Glow")
          (Utilities|FlowControl|Delay 0.2)
          (Rendering|Material|SetMaterial _cube_2 0 "/Game/TeamFolders/Martin/Materials/M_Red_Glow.M_Red_Glow")
          (Rendering|Material|SetMaterial _cube_2 2 "/Game/TeamFolders/Martin/Materials/M_Red_Glow.M_Red_Glow"))
        (:then_1
          (bind _outactors (Actor|GetAllActorsOfClass "/Game/TeamFolders/Martin/Assets/Cannon/Cannon_BP.Cannon_BP_C"))
          (Game|SpawnActorfromClass "/Game/TeamFolders/Martin/Assets/Cannon/CannonBallDK_BP.CannonBallDK_BP_C" (Math|Conversions|ToTransform(Vector) (Transformation|GetWorldLocation (Variables|/Game/TeamFolders/Martin/Assets/Cannon/Cannon_BP.Cannon_BP_C|GetBarrelArrow (Utilities|Array|Get(acopy) _outactors)))) "Undefined" 0 0))))))

(event EventBeginPlay
  ;[1 1 1] Spawns cannon onto plate
  (Game|SpawnActorfromClass "/Game/TeamFolders/Martin/Assets/Cannon/Cannon_BP.Cannon_BP_C" (Math|Conversions|ToTransform(Vector) (Transformation|GetWorldLocation (Variables|Default|GetBarrelSpawnPoint))) "Undefined" 0 0))

(fn ConstructionScript)