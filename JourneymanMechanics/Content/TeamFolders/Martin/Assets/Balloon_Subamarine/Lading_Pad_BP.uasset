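; Landing pad for the Balloon Submarine that hands player control to Mario when the balloon lands on it.
; An overlap on the charge plate box casts to the submarine, then possesses the first Mario character found in the world with the first player controller.
; It also turns the pressure pad red and briefly stops the submarine's movement, with a flag making it single use.
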(event OnComponentBeginOverlap(Box_Charge_Plate)
  (params (OverlappedComponent :type Primitive%20Component%20Object%20Reference) (OtherActor :type Actor%20Object%20Reference) (OtherComp :type Primitive%20Component%20Object%20Reference) (OtherBodyIndex :type Integer) (bFromSweep :type Boolean) (SweepResult :type Hit%20Result%20Structure%20%28by%20ref%29))
  ;[1 1 1] Posses Mario when Balloon lands on pad, then change pad to red. 1 time use.
  (bind _asballoon_submarine (Utilities|Casting|CastToBalloon_Submarine OtherActor))
  (if (not (Variables|Default|GetPadLandedOn))
    (bind _outactors (Actor|GetAllActorsOfClass "/Game/SideScrollerBP/Blueprints/Mario_Character.Mario_Character_C"))
    (Pawn|Possess (Game|GetPlayerController 0) (Utilities|Array|Get(acopy) _outactors))
    (Rendering|Material|SetMaterial (Variables|Default|GetPressurePad) 0 "/Game/TeamFolders/Martin/Materials/M_Red_Glow.M_Red_Glow")
    (Variables|Default|SetPadLandedOn true)
    (Default|StopMovementBriefly _asballoon_submarine)))

(fn ConstructionScript)