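; DoorCube1_BP is a door cube actor that removes itself once a three-block button puzzle is solved.
; Three custom events, one per block turning green, each add a point to a completion counter.
; Tick polls that counter and, once it reaches three, destroys the actor after a short delay.
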(event Custom|Completed1_3
  ;[1 1 1] Add 1 point for when block 3 is turned green
  (Variables|Default|SetCompelte (+ (Variables|Default|GetCompelte) 1.0)))

(event Custom|Completed1_1
  ;[1 1 1] Add 1 point for when block 1 is turned green
  (Variables|Default|SetCompelte (+ (Variables|Default|GetCompelte) 1.0)))

(event Custom|Completed1_2
  ;[1 1 1] Add 1 point for when block 2 is turned green
  (Variables|Default|SetCompelte (+ (Variables|Default|GetCompelte) 1.0)))

(event EventTick
  (params (DeltaSeconds :type Float%20%28single-precision%29))
  ;[1 1 1] Comment
  (if (>= (Variables|Default|GetCompelte) 3.0)
    (Utilities|FlowControl|Delay 0.2)
    (Actor|DestroyActor)))

(fn ConstructionScript)