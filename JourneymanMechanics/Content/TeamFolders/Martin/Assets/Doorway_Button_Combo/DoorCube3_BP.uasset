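; DoorCube3_BP is a door cube in a three-button doorway combo that removes itself once all three blocks are turned green.
; Three custom events, one per block, each add a point to a Complete counter, with no guard against the same block counting twice.
; Tick polls the counter and, once it reaches three, destroys the actor after a short delay.
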(event Custom|Completed3_3
  ;[1 1 1] Add 1 point for when block 3 is turned green
  (Variables|Default|SetComplete (+ (Variables|Default|GetComplete) 1.0)))

(event Custom|Completed3_1
  ;[1 1 1] Add 1 point for when block 1 is turned green
  (Variables|Default|SetComplete (+ (Variables|Default|GetComplete) 1.0)))

(event Custom|Completed3_2
  ;[1 1 1] Add 1 point for when block 2 is turned green
  (Variables|Default|SetComplete (+ (Variables|Default|GetComplete) 1.0)))

(event EventTick
  (params (DeltaSeconds :type Float%20%28single-precision%29))
  ;[1 1 1] Comment
  (if (>= (Variables|Default|GetComplete) 3.0)
    (Utilities|FlowControl|Delay 0.2)
    (Actor|DestroyActor)))

(fn ConstructionScript)