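; Mario-style coin block that spawns a coin each time a Mario_Character hits it from an overlap.
; BoxCollision overlaps increment a hit counter and spawn Coin_BP at the Arrow component's location.
; On the fifth hit the Cube switches to a brown material after a short delay to look used up.
; Nothing disables the box, so later hits still spawn coins despite comments saying it breaks.
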(event OnComponentBeginOverlap(BoxCollision)
  (params (OverlappedComponent :type Primitive%20Component%20Object%20Reference) (OtherActor :type Actor%20Object%20Reference) (OtherComp :type Primitive%20Component%20Object%20Reference) (OtherBodyIndex :type Integer) (bFromSweep :type Boolean) (SweepResult :type Hit%20Result%20Structure%20%28by%20ref%29))
  ;[1 1 1] When character hits box, it will activate custom events depending on which variable was selected from event begin play, on the 5th hit, the box will destroy
  (Utilities|Casting|CastToMario_Character OtherActor)
  (Variables|Default|SetBoxHitAmount (+ (Variables|Default|GetBoxHitAmount) 1.0))
  (if (== (Variables|Default|GetBoxHitAmount) 5.0)
    (CallFunction|CoinBox)
    (Utilities|FlowControl|Delay 0.4)
    (Rendering|Material|SetMaterial (Variables|Default|Get?Cube) 0 "/Game/TeamFolders/Martin/Materials/M_Brown.M_Brown")
    (else
      (CallFunction|CoinBox))))

(event Custom|CoinBox
  ;[1 1 1] Good box, will produce 5 coins then the box will break and no longer be usable
  (Game|SpawnActorfromClass "/Game/TeamFolders/Martin/Assets/FloatingBlocks/Coin_BP.Coin_BP_C" (Math|Transform|MakeTransform (Transformation|GetWorldLocation (Variables|Default|GetArrow)) "0, 0, 0" "1,1,1") "Undefined" 0 0))

(fn ConstructionScript)