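; Floating Mario-style hit block that randomly becomes a coin, enemy or power-up box when play begins.
; A random MultiGate in BeginPlay sets one type flag, with extra pins serving as a way to weight the odds.
; When Mario_Character overlaps BoxCollision, the flag selects a custom event that spawns the matching actor at the Arrow.
; Coin boxes destroy themselves shortly after the fifth hit, while enemy and power-up boxes do so after one.
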(event OnComponentBeginOverlap(BoxCollision)
  (params (OverlappedComponent :type Primitive%20Component%20Object%20Reference) (OtherActor :type Actor%20Object%20Reference) (OtherComp :type Primitive%20Component%20Object%20Reference) (OtherBodyIndex :type Integer) (bFromSweep :type Boolean) (SweepResult :type Hit%20Result%20Structure%20%28by%20ref%29))
  ;[1 1 1] When character hits box, it will activate custom events depending on which variable was selected from event begin play
  (Utilities|Casting|CastToMario_Character OtherActor)
  (Utilities|FlowControl|Sequence
    (:then_0
      ;;[1 1 1] Coin Mechanics
      (if (Variables|CoinBoxes|GetCoinBoxChosen)
        (Variables|Default|SetBoxHitAmount (+ (Variables|Default|GetBoxHitAmount) 1.0))
        (if (== (Variables|Default|GetBoxHitAmount) 5.0)
          (CallFunction|CoinBox)
          (Utilities|FlowControl|Delay 0.4)
          (Actor|DestroyActor)
          (else
            (CallFunction|CoinBox)))))
    (:then_1
      ;;[1 1 1] Enemy Mechanics
      (if (Variables|CoinBoxes|GetEnemyBoxChosen)
        (CallFunction|EnemyBox)
        (Utilities|FlowControl|Delay 0.3)
        (Actor|DestroyActor)))
    (:then_2
      ;;[1 1 1] PUP Mechanics
      (if (Variables|CoinBoxes|GetPUPBoxChosen)
        (CallFunction|PUPBox)
        (Utilities|FlowControl|Delay 0.3)
        (Actor|DestroyActor)))))

(event Custom|CoinBox
  ;[1 1 1] Coin box, will produce 5 coins then the box will break and no longer be usable
  (Game|SpawnActorfromClass "/Game/TeamFolders/Martin/Assets/FloatingBlocks/Coin_BP.Coin_BP_C" (Math|Transform|MakeTransform (Transformation|GetWorldLocation (Variables|Default|GetArrow)) "0, 0, 0" "1,1,1") "Undefined" 0 0))

(event Custom|PUPBox
  ;[1 1 1] PowerUp box (PUP), will produce 1 PUP then the box will break and no longer be usable
  (Game|SpawnActorfromClass "/Game/TeamFolders/Martin/Assets/FloatingBlocks/Powerup_BP.Powerup_BP_C" (Math|Transform|MakeTransform (Transformation|GetWorldLocation (Variables|Default|GetArrow)) "0, 0, 0" "1,1,1") "Undefined" 0 0))

(event Custom|EnemyBox
  ;[1 1 1] Enemy box, will produce 1 enemy then the box will break and no longer be usable
  (Game|SpawnActorfromClass "/Game/TeamFolders/Martin/Assets/FloatingBlocks/Enemy_BP.Enemy_BP_C" (Math|Transform|MakeTransform (Transformation|GetWorldLocation (Variables|Default|GetArrow)) "0, 0, 0" "1,1,1") "Undefined" 0 0))

(event EventBeginPlay
  ;[1 1 1] Chooses if the box will be a coin, PUP or Enemy box. If you want more of a chance for it to be a certian box i.e. more chances of coin box appeaing, just add more pins to the MultiGate and then add more Coin Box Chosen set nodes.
  (Utilities|FlowControl|MultiGate true false -1
    (:Out%200
      (Variables|CoinBoxes|SetCoinBoxChosen true))
    (:Out%201
      (Variables|CoinBoxes|SetEnemyBoxChosen true))
    (:Out%202
      (Variables|CoinBoxes|SetPUPBoxChosen true))))

(fn ConstructionScript)