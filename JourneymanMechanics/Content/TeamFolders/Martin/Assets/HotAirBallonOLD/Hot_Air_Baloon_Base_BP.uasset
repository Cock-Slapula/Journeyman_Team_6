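; Hot air balloon base that Mario_Character inflates by repeatedly jumping on a pressure pad, then boards to fly.
; Overlaps on the pad increment a counter that scales the balloon through six stages and toggle the pad between green and red glow.
; The final stage destroys the basket door.
; Entering the inflated basket hides the character, spawns HotAirBallon_BP, possesses the first instance found and removes the placeholder balloon components.
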(event OnComponentBeginOverlap(Box_Charge_Plate)
  (params (OverlappedComponent :type Primitive%20Component%20Object%20Reference) (OtherActor :type Actor%20Object%20Reference) (OtherComp :type Primitive%20Component%20Object%20Reference) (OtherBodyIndex :type Integer) (bFromSweep :type Boolean) (SweepResult :type Hit%20Result%20Structure%20%28by%20ref%29))
  (bind _sphere (Variables|Default|GetSphere))
  ;[1 1 1] When the player jumps onto the pressure pad/button, it will inflate the balloon in 6 stages (must jump on the button 6 times). The colour of the pad/button will change to green when they successfully jump onto it. Once the balloon is fully inflated, the door to the basket will destroy allowing access.
  (Utilities|Casting|CastToMario_Character OtherActor)
  (Variables|Default|SetJumpedON (+ (Variables|Default|GetJumpedON) 1.0))
  (Rendering|Material|SetMaterial (Variables|Default|GetPressurePad) 0 "/Game/TeamFolders/Martin/Materials/M_Green_Glow.M_Green_Glow")
  (Utilities|FlowControl|Sequence
    (:then_0
      (if (== (Variables|Default|GetJumpedON) 1.0)
        (Transformation|SetRelativeScale3D _sphere "0.500000,0.500000,1.250000")
        (Variables|Default|SetInflated1 true)))
    (:then_1
      (if (== (Variables|Default|GetJumpedON) 2.0)
        (if (Variables|Default|GetInflated1)
          (Transformation|SetRelativeScale3D _sphere "0.750000,0.750000,1.250000")
          (Variables|Default|SetInflated2 true))))
    (:then_2
      (if (== (Variables|Default|GetJumpedON) 3.0)
        (if (Variables|Default|GetInflated2)
          (Transformation|SetRelativeScale3D _sphere "1.000000,1.000000,1.250000")
          (Variables|Default|SetInflated3 true))))
    (:then_3
      (if (== (Variables|Default|GetJumpedON) 4.0)
        (if (Variables|Default|GetInflated3)
          (Transformation|SetRelativeScale3D _sphere "1.000000,1.250000,1.250000")
          (Variables|Default|SetInflated4 true))))
    (:then_4
      (if (== (Variables|Default|GetJumpedON) 5.0)
        (if (Variables|Default|GetInflated4)
          (Transformation|SetRelativeScale3D _sphere "1.000000,1.500000,1.250000")
          (Variables|Default|SetInflated5 true))))
    (:then_5
      (if (== (Variables|Default|GetJumpedON) 6.0)
        (if (Variables|Default|GetInflated5)
          (Transformation|SetRelativeScale3D _sphere "1.000000,2.000000,1.250000")
          (Variables|Default|SetInflated6 true)
          (Components|DestroyComponent (Variables|Default|GetBasketDoor)))))))

(event OnComponentEndOverlap(Box_Charge_Plate)
  (params (OverlappedComponent :type Primitive%20Component%20Object%20Reference) (OtherActor :type Actor%20Object%20Reference) (OtherComp :type Primitive%20Component%20Object%20Reference) (OtherBodyIndex :type Integer))
  ;[1 1 1] When the player jumps onto the pressure pad/button, it will inflate the balloon in 6 stages (must jump on the button 6 times). The colour of the pad/button will change to green when they successfully jump onto it. Once the balloon is fully inflated, the door to the basket will destroy allowing access.
  (Utilities|Casting|CastToMario_Character OtherActor)
  (Rendering|Material|SetMaterial (Variables|Default|GetPressurePad) 0 "/Game/TeamFolders/Martin/Materials/M_Red_Glow.M_Red_Glow"))

(event OnComponentBeginOverlap(Box_Balloon_Basket)
  (params (OverlappedComponent :type Primitive%20Component%20Object%20Reference) (OtherActor :type Actor%20Object%20Reference) (OtherComp :type Primitive%20Component%20Object%20Reference) (OtherBodyIndex :type Integer) (bFromSweep :type Boolean) (SweepResult :type Hit%20Result%20Structure%20%28by%20ref%29))
  ;[1 1 1] If the balloon is fully inflated and the character stands on the balloon basket, it will disable the players input and then trigger the take control of the hot air ballon event.
  (bind _asmario_character (Utilities|Casting|CastToMario_Character OtherActor))
  (if (Variables|Default|GetInflated6)
    (Rendering|SetActorHiddenInGame _asmario_character true)
    (Game|SpawnActorfromClass "/Game/TeamFolders/Martin/Assets/HotAirBallonOLD/HotAirBallon_BP.HotAirBallon_BP_C" (Math|Conversions|ToTransform(Vector) (Transformation|GetWorldLocation (Variables|Default|GetCube))) "Undefined" 0 0)
    (bind _outactors (Actor|GetAllActorsOfClass "/Game/TeamFolders/Martin/Assets/HotAirBallonOLD/HotAirBallon_BP.HotAirBallon_BP_C"))
    (Pawn|Possess (Game|GetPlayerController 0) (Utilities|Array|Get(acopy) _outactors))
    (Components|DestroyComponent (Variables|Default|GetSphere))
    (else
      (Development|PrintString "Inflate the balloon!"))))

(fn ConstructionScript)