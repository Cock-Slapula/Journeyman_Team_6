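; Player-controlled hot air balloon pawn that hands control back to Mario_Character on landing.
; W and S move it up and down, A and D along the world Y axis, via key-toggled gates pulsed each Tick.
; Overlapping a landing pad possesses the first Mario_Character, teleports it to ArrowFloor and unhides it.
; Lean events rotate the Sphere and Cube but are disconnected and marked as needing fixes.
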(event OnComponentBeginOverlap(Box)
  (params (OverlappedComponent :type Primitive%20Component%20Object%20Reference) (OtherActor :type Actor%20Object%20Reference) (OtherComp :type Primitive%20Component%20Object%20Reference) (OtherBodyIndex :type Integer) (bFromSweep :type Boolean) (SweepResult :type Hit%20Result%20Structure%20%28by%20ref%29))
  ;[1 1 1] When the balloon collides with the landing pad, it will take control back of the player character
  (Utilities|Casting|CastToHot_Air_Baloon_Lading_Pad_BP OtherActor)
  (bind _outactors (Actor|GetAllActorsOfClass "/Game/SideScrollerBP/Blueprints/Mario_Character.Mario_Character_C"))
  (Pawn|Possess (Game|GetPlayerController 0) (Utilities|Array|Get(acopy) _outactors))
  (Transformation|Teleport (Utilities|Array|Get(acopy) _outactors) (Transformation|GetWorldLocation (Variables|Default|GetArrow-Floor)) "0, 0, 0")
  (Rendering|SetActorHiddenInGame (Utilities|Array|Get(acopy) _outactors) false))

(event Custom|LeanLeft
  ;[1 1 1] THIS NEEDS FIXING!!!!!
  ;;[1 1 1] Leans the balloon to the left when pressing A
  (Utilities|FlowControl|Sequence
    (:then_0
      (Transformation|SetWorldRotation (Variables|Default|GetSphere) "0.000000,0.000000,20.000000" false false))))

(event Custom|LeanRight
  ;[1 1 1] THIS NEEDS FIXING!!!!!
  ;;[1 1 1] Leans the balloon to the right when pressing D
  (Utilities|FlowControl|Sequence
    (:then_0
      (Transformation|SetWorldRotation (Variables|Default|GetSphere) "0.000000,0.000000,-20.000000" false false))))

(event Custom|NormalRotation
  ;[1 1 1] THIS NEEDS FIXING!!!!!
  ;;[1 1 1] Comment
  (Utilities|FlowControl|Sequence
    (:then_0
      (Transformation|SetWorldRotation (Variables|Default|GetSphere) "0, 0, 0" false false))))

(event EventTick
  (params (DeltaSeconds :type Float%20%28single-precision%29))
  ;[1 1 1] Allows the hot air balloon to move with WASD (change this later for the joystick). The custom events not connected are for the balloon to lean as it moves though they need fixing!!!
  (Utilities|FlowControl|Sequence
    (:then_0
      (Utilities|FlowControl|Gate true
        (:Exit
          (Pawn|Input|AddMovementInput "0,0.000000,1.000000" 1.0 false))))
    (:then_1
      (Utilities|FlowControl|Gate true
        (:Exit
          (Pawn|Input|AddMovementInput "0,1.000000,0.000000" 1.0 false))))
    (:then_2
      (Utilities|FlowControl|Gate true
        (:Exit
          (Pawn|Input|AddMovementInput "0.000000,-1.000000, 0" 1.0 false))))
    (:then_3
      (Utilities|FlowControl|Gate true
        (:Exit
          (Pawn|Input|AddMovementInput "0.000000,0.000000,-1.000000" 1.0 false))))))

(event Input|KeyboardEvents|W
  (params (Key :type Key%20Structure))
  ;[1 1 1] Allows the hot air balloon to move with WASD (change this later for the joystick). The custom events not connected are for the balloon to lean as it moves though they need fixing!!!
  (:Pressed
    (Utilities|FlowControl|Gate true) ; enters at Open
  )
  (:Released
    (Utilities|FlowControl|Gate true) ; enters at Close
  ))

(event Input|KeyboardEvents|A
  (params (Key :type Key%20Structure))
  ;[1 1 1] Allows the hot air balloon to move with WASD (change this later for the joystick). The custom events not connected are for the balloon to lean as it moves though they need fixing!!!
  (:Pressed
    (Utilities|FlowControl|Gate true) ; enters at Open
  )
  (:Released
    (Utilities|FlowControl|Sequence
      (:then_0
        (Utilities|FlowControl|Gate true) ; enters at Close
      ))))

(event Input|KeyboardEvents|D
  (params (Key :type Key%20Structure))
  ;[1 1 1] Allows the hot air balloon to move with WASD (change this later for the joystick). The custom events not connected are for the balloon to lean as it moves though they need fixing!!!
  (:Pressed
    (Utilities|FlowControl|Gate true) ; enters at Open
  )
  (:Released
    (Utilities|FlowControl|Sequence
      (:then_0
        (Utilities|FlowControl|Gate true) ; enters at Close
      ))))

(event Input|KeyboardEvents|S
  (params (Key :type Key%20Structure))
  ;[1 1 1] Allows the hot air balloon to move with WASD (change this later for the joystick). The custom events not connected are for the balloon to lean as it moves though they need fixing!!!
  (:Pressed
    (Utilities|FlowControl|Gate true) ; enters at Open
  )
  (:Released
    (Utilities|FlowControl|Gate true) ; enters at Close
  ))

(fn ConstructionScript)