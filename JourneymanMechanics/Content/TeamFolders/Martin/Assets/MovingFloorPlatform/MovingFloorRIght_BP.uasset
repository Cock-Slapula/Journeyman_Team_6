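; Moving floor platform Blueprint that shuttles a platform back and forth between its starting position and an end marker.
; On BeginPlay it caches both world locations, then two timelines lerp the platform out and back without sweep.
; Each timeline's Update pin, rather than Finished, feeds a four-second Delay that starts the opposite timeline, so the cycle repeats on timing from each move's start.
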(event EventBeginPlay
  (bind _platform (Variables|Default|GetPlatform))
  ;[1 1 1] Get locations
  (Utilities|FlowControl|Sequence
    (:then_0
      (Variables|Default|SetStart_Location (Transformation|GetWorldLocation (Variables|Default|GetPlatform)))
      (Variables|Default|SetEnd_Location (Transformation|GetWorldLocation (Variables|Default|GetEndLocation)))
      (bind _newtrack_0 (Timeline|Timeline_0 PlayFromStart)
        (:Update
          (Transformation|SetWorldLocation _platform (Math|Vector|Lerp(Vector) (Variables|Default|GetStart_Location) (Variables|Default|GetEnd_Location) _newtrack_0) false false)
          (Utilities|FlowControl|Delay 4.0)
          (bind _newtrack_0_2 (Timeline|Timeline_1 PlayFromStart)
            (:Update
              (Transformation|SetWorldLocation _platform (Math|Vector|Lerp(Vector) (Variables|Default|GetEnd_Location) (Variables|Default|GetStart_Location) _newtrack_0_2) false false)
              (Utilities|FlowControl|Delay 4.0)
              (Timeline|Timeline_0 PlayFromStart))))))))

(fn ConstructionScript)