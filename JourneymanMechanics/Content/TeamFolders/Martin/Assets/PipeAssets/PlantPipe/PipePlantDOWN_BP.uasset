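; A Mario-style pipe plant hazard that endlessly rises out of and sinks back down, killing the player on contact.
; On BeginPlay it caches the plant's position and an arrow's position as endpoints, then loops raise and lower moves with fixed delays.
; Two timelines, one played forward and one in reverse, lerp the plant's relative location between the endpoints.
; A sphere overlap destroys any overlapping Mario_Character.
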(event OnComponentBeginOverlap(Sphere)
  (params (OverlappedComponent :type Primitive%20Component%20Object%20Reference) (OtherActor :type Actor%20Object%20Reference) (OtherComp :type Primitive%20Component%20Object%20Reference) (OtherBodyIndex :type Integer) (bFromSweep :type Boolean) (SweepResult :type Hit%20Result%20Structure%20%28by%20ref%29))
  ;[1 1 1] Kill player on contact
  (bind _asmario_character (Utilities|Casting|CastToMario_Character OtherActor))
  (Actor|DestroyActor _asmario_character))

(event Custom|MoveplantUP
  ;[1 1 1] Moves plant up
  (bind _newtrack_0 (Timeline|Timeline_0 PlayFromStart)
    (:Update
      (Transformation|SetRelativeLocation (Variables|Default|GetPlant) (Math|Vector|Lerp(Vector) (Variables|Default|GetStartLocation) (Variables|Default|GetEndLocation) _newtrack_0) false false))))

(event Custom|MoveplantDown
  ;[1 1 1] Moves plant back down
  (bind _newtrack_0 (Timeline|Timeline_1 ReverseFromEnd)
    (:Update
      (Transformation|SetRelativeLocation (Variables|Default|GetPlant) (Math|Vector|Lerp(Vector) (Variables|Default|GetStartLocation) (Variables|Default|GetEndLocation) _newtrack_0) false false))))

(event EventBeginPlay
  ;[1 1 1] When the plant spawns, it will set 2 loctions, the start location is the plant itself, the end location is the arrow above the plant
  (Utilities|FlowControl|Sequence
    (:then_0
      ;;[1 1 1] Plant fully DOWN
      (Variables|Default|SetStartLocation (Variables|/Script/Engine.SceneComponent|GetRelativeLocation (Variables|Default|GetPlant))))
    (:then_1
      ;;[1 1 1] Plant fully UP
      (Variables|Default|SetEndLocation (Variables|/Script/Engine.SceneComponent|GetRelativeLocation (Variables|Default|GetArrow))))
    (:then_2
      (CallFunction|MoveplantUP :!label _label)
      (Utilities|FlowControl|Delay 2.3)
      (CallFunction|MoveplantDown)
      (Utilities|FlowControl|Delay 2.3)
      (goto _label))))

(fn ConstructionScript)