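; Changeable world-warp block that is solid in either the bright or dark world and shown as non-colliding glass in the other.
; WorldWarp toggles LightMode and DarkMode, which set collision, material and CanDie from Block1Bright.
; A Mario overlap on Box moves the block to the opposite world with a Timeline bump and delayed collision shutoff.
; Box8 kills an overlapping Mario while CanDie is true, catching players inside mid-warp.
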(event OnComponentBeginOverlap(Box)
  (params (OverlappedComponent :type Primitive%20Component%20Object%20Reference) (OtherActor :type Actor%20Object%20Reference) (OtherComp :type Primitive%20Component%20Object%20Reference) (OtherBodyIndex :type Integer) (bFromSweep :type Boolean) (SweepResult :type Hit%20Result%20Structure%20%28by%20ref%29))
  (bind _z (Variables|Default|GetZ))
  (bind _y (Variables|Default|GetY))
  ;[1 1 1] Block hit animation and changing world block exists in
  (Utilities|FlowControl|Sequence
    (:then_0
      (goto _label Reset))
    (:then_1
      (Utilities|Casting|CastToMario_Character OtherActor)
      (if (Variables|Default|GetMap_State_Dark)
        (Variables|Default|SetBlock1%20%28Bright%29 true)
        (else
          (Variables|Default|SetBlock1%20%28Bright%29 false)))
      (Rendering|Material|SetMaterial (Variables|Default|GetBlock_1) 0 "/Game/TeamFolders/Aaron/Lvl3_AM_001/AaronM/M_Glass.M_Glass")
      (bind _newtrack_0 (Timeline|Timeline_0 Play)
        (:Update
          (Transformation|SetRelativeLocation (Variables|Default|GetBlock_1) (Math|Vector|Lerp(Vector) (Math|Vector|MakeVector 0.0 _y _z) (Math|Vector|MakeVector 0.0 _y (+ _z 2e+01)) _newtrack_0) false false)
          (Utilities|FlowControl|Delay 0.13)
          (Collision|SetActorEnableCollision false)
          (Utilities|FlowControl|DoOnce false :!label _label
            (:Completed
              (Timeline|Timeline_0 Reverse))))))))

(event OnComponentBeginOverlap(Box8)
  (params (OverlappedComponent :type Primitive%20Component%20Object%20Reference) (OtherActor :type Actor%20Object%20Reference) (OtherComp :type Primitive%20Component%20Object%20Reference) (OtherBodyIndex :type Integer) (bFromSweep :type Boolean) (SweepResult :type Hit%20Result%20Structure%20%28by%20ref%29))
  ;[1 1 1] Player can die if overlapped with the hitbox mid world warp
  (if (Variables|Default|Getcan%20die)
    (bind _asmario_character (Utilities|Casting|CastToMario_Character OtherActor))
    (Default|IsDead _asmario_character)))

(event Custom|World%20Warp
  ;[1 1 1] Checking which world the player is currently in and triggering the change
  (if (Variables|Default|GetMap_State_Dark)
    (CallFunction|LightMode)
    (else
      (CallFunction|DarkMode))))

(event Custom|Light%20Mode
  (bind _block_1 (Variables|Default|GetBlock_1))
  ;[1 1 1] Changes asset properties depending on which mode has been triggered
  (Variables|Default|SetMap_State_Dark false)
  (if (Variables|Default|GetBlock1%20%28Bright%29)
    (Variables|Default|Setcan%20die true)
    (Collision|SetActorEnableCollision true)
    (Rendering|Material|SetMaterial _block_1 0 0)
    (else
      (Variables|Default|Setcan%20die false)
      (Collision|SetActorEnableCollision false)
      (Rendering|Material|SetMaterial _block_1 0 "/Game/TeamFolders/Aaron/Lvl3_AM_001/AaronM/M_Glass.M_Glass"))))

(event Custom|Dark%20Mode
  (bind _block_1 (Variables|Default|GetBlock_1))
  ;[1 1 1] Changes asset properties depending on which mode has been triggered
  (Variables|Default|SetMap_State_Dark true)
  (if (Variables|Default|GetBlock1%20%28Bright%29)
    (Variables|Default|Setcan%20die false)
    (Collision|SetActorEnableCollision false)
    (Rendering|Material|SetMaterial _block_1 0 "/Game/TeamFolders/Aaron/Lvl3_AM_001/AaronM/M_Glass.M_Glass")
    (else
      (Variables|Default|Setcan%20die true)
      (Collision|SetActorEnableCollision true)
      (Rendering|Material|SetMaterial _block_1 0 0))))

(event EventBeginPlay
  (bind _block_1 (Variables|Default|GetBlock_1))
  (bind _relativelocation (Variables|/Script/Engine.SceneComponent|GetRelativeLocation _block_1))
  ;[1 1 1] Getting start Coords for animation
  (Variables|Default|SetY (.y _relativelocation))
  (Variables|Default|SetZ (.z _relativelocation)))

(event Collision|EventActorBeginOverlap
  (params (OtherActor :type Actor%20Object%20Reference)))

(event EventTick
  (params (DeltaSeconds :type Float%20%28single-precision%29)))

(fn ConstructionScript)