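; Block that exists in both the Dark and Light world states, staying visible and solid in each.
; Its ChangeState event switches on the current state and changes only the mesh material: M_White in Dark, DarkWorld in Light.
; The construction script just calls the parent's.
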(event EventChangeState
  (params (Current%20state :type E_WorldSwitch%20Enum :default "NewEnumerator0"))
  (switch Utilities|FlowControl|Switch|SwitchonE_WorldSwitch Current%20state
    (:NewEnumerator0
      (Rendering|SetVisibility (Variables|Default|GetStaticMesh) true false)
      (Collision|SetCollisionEnabled (Variables|Default|GetStaticMesh) "QueryAndPhysics")
      (Rendering|Material|SetMaterial (Variables|Default|GetStaticMesh) 0 "/Game/TeamFolders/Martin/Materials/M_White.M_White"))
    (:NewEnumerator1
      (Rendering|SetVisibility (Variables|Default|GetStaticMesh) true false)
      (Collision|SetCollisionEnabled (Variables|Default|GetStaticMesh) "QueryAndPhysics")
      (Rendering|Material|SetMaterial (Variables|Default|GetStaticMesh) 0 "/Game/SideScrollerBP/Materials/DarkWorld.DarkWorld"))))

(fn ConstructionScript
  (|CallParentFunction))