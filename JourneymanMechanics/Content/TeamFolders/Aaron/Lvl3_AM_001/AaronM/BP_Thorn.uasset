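; BP_Thorn is a thorn hazard that is dangerous only in the Dark world state.
; ChangeState switches it between an active white look in Dark, with the KillBox collision on, and a harmless glass look in Light, with it off.
; The mesh stays visible and non-colliding in both states.
; A Mario_Character overlapping the KillBox currently only prints a death message, with no actual kill logic.
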(event OnComponentBeginOverlap(KillBox)
  (params (OverlappedComponent :type Primitive%20Component%20Object%20Reference) (OtherActor :type Actor%20Object%20Reference) (OtherComp :type Primitive%20Component%20Object%20Reference) (OtherBodyIndex :type Integer) (bFromSweep :type Boolean) (SweepResult :type Hit%20Result%20Structure%20%28by%20ref%29))
  ;[1 1 1] Kills PLayer
  (Utilities|Casting|CastToMario_Character OtherActor)
  (Development|PrintString "DEAD"))

(event EventChangeState
  (params (Current%20state :type E_WorldSwitch%20Enum :default "NewEnumerator0"))
  (switch Utilities|FlowControl|Switch|SwitchonE_WorldSwitch Current%20state
    (:NewEnumerator0
      (Rendering|SetVisibility (Variables|Default|GetStaticMesh) true false)
      (Collision|SetCollisionEnabled (Variables|Default|GetStaticMesh) "NoCollision")
      (Rendering|Material|SetMaterial (Variables|Default|GetStaticMesh) 0 "/Game/TeamFolders/Martin/Materials/M_White.M_White")
      (Collision|SetCollisionEnabled (Variables|Default|GetKill%20Box) "QueryAndPhysics"))
    (:NewEnumerator1
      (Rendering|SetVisibility (Variables|Default|GetStaticMesh) true false)
      (Collision|SetCollisionEnabled (Variables|Default|GetStaticMesh) "NoCollision")
      (Rendering|Material|SetMaterial (Variables|Default|GetStaticMesh) 0 "/Game/TeamFolders/Aaron/Lvl3_AM_001/AaronM/M_Glass.M_Glass"))))

(fn ConstructionScript
  (|CallParentFunction))