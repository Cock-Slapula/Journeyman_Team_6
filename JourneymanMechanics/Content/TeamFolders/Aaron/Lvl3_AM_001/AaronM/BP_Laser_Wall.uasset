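; Laser wall hazard that reacts to Dark/Light world changes: glass with no laser or kill collision in Dark, solid with a cycling laser in Light.
; First switch to Light starts an endless delay loop that blinks a faster warning, fires the beam briefly, then resets.
; InLight, set inversely to its name, suppresses loop activation in Dark.
; Mario overlaps set a DontSwap flag or, in KillZone, only print "DEAD".
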(event OnComponentBeginOverlap(Don'tSwap)
  (params (OverlappedComponent :type Primitive%20Component%20Object%20Reference) (OtherActor :type Actor%20Object%20Reference) (OtherComp :type Primitive%20Component%20Object%20Reference) (OtherBodyIndex :type Integer) (bFromSweep :type Boolean) (SweepResult :type Hit%20Result%20Structure%20%28by%20ref%29))
  ;[1 1 1] If Collided doesn't swap worlds
  (Utilities|Casting|CastToMario_Character OtherActor)
  (Variables|Default|SetDontSwap true))

(event OnComponentEndOverlap(Don'tSwap)
  (params (OverlappedComponent :type Primitive%20Component%20Object%20Reference) (OtherActor :type Actor%20Object%20Reference) (OtherComp :type Primitive%20Component%20Object%20Reference) (OtherBodyIndex :type Integer))
  ;[1 1 1] If Collided doesn't swap worlds
  (Utilities|Casting|CastToMario_Character OtherActor)
  (Variables|Default|SetDontSwap false))

(event OnComponentBeginOverlap(KillZone)
  (params (OverlappedComponent :type Primitive%20Component%20Object%20Reference) (OtherActor :type Actor%20Object%20Reference) (OtherComp :type Primitive%20Component%20Object%20Reference) (OtherBodyIndex :type Integer) (bFromSweep :type Boolean) (SweepResult :type Hit%20Result%20Structure%20%28by%20ref%29))
  (Utilities|Casting|CastToMario_Character OtherActor)
  (Development|PrintString "DEAD"))

(event EventChangeState
  (params (Current%20state :type E_WorldSwitch%20Enum :default "NewEnumerator0"))
  (bind _cube (Variables|Default|GetCube))
  ;[1 1 1] Laser Sequence (Keeps going no matter what world the player is in)
  (switch Utilities|FlowControl|Switch|SwitchonE_WorldSwitch Current%20state
    (:NewEnumerator0
      (Rendering|SetVisibility (Variables|Default|GetStaticMesh) true false)
      (Collision|SetCollisionEnabled (Variables|Default|GetStaticMesh) "NoCollision")
      (Rendering|Material|SetMaterial (Variables|Default|GetStaticMesh) 0 "/Game/TeamFolders/Aaron/Lvl3_AM_001/AaronM/M_Glass.M_Glass")
      (Rendering|SetVisibility (Variables|Default|GetCube) false false)
      (Variables|Default|SetInLight true))
    (:NewEnumerator1
      (if (Variables|Default|GetLaserActive)
        (Rendering|SetVisibility _cube true false)
        (Collision|SetCollisionEnabled (Variables|Default|GetKill%20Zone) "QueryAndPhysics")
        (Rendering|Material|SetMaterial _cube 0 "/Engine/VREditor/LaserPointer/LaserPointerMaterial.LaserPointerMaterial")
        (Rendering|Material|SetMaterial (Variables|Default|GetStaticMesh) 0 "/Game/TeamFolders/Martin/Materials/M_Red_Dark.M_Red_Dark")
        (else
          (Rendering|SetVisibility (Variables|Default|GetCube) false false)
          (Rendering|Material|SetMaterial (Variables|Default|GetStaticMesh) 0 "/Game/SideScrollerBP/Materials/DarkWorld.DarkWorld")
          (Collision|SetCollisionEnabled (Variables|Default|GetKill%20Zone) "NoCollision")))
      (Rendering|SetVisibility (Variables|Default|GetStaticMesh) true false)
      (Collision|SetCollisionEnabled (Variables|Default|GetStaticMesh) "QueryAndPhysics")
      (Variables|Default|SetInLight false)
      (Utilities|FlowControl|DoOnce false
        (:Completed
          (Utilities|FlowControl|Delay (Variables|Default|GetDelay) :!label _label)
          (if (Variables|Default|GetInLight)
            _
            (else
              (Rendering|Material|SetMaterial (Variables|Default|GetStaticMesh) 0 "/Game/TeamFolders/Martin/Materials/M_Red_Dark.M_Red_Dark")))
          (Utilities|FlowControl|Delay 0.75)
          (if (Variables|Default|GetInLight)
            _
            (else
              (Rendering|Material|SetMaterial (Variables|Default|GetStaticMesh) 0 "/Game/SideScrollerBP/Materials/DarkWorld.DarkWorld")))
          (Utilities|FlowControl|Delay 0.75)
          (if (Variables|Default|GetInLight)
            _
            (else
              (Rendering|Material|SetMaterial (Variables|Default|GetStaticMesh) 0 "/Game/TeamFolders/Martin/Materials/M_Red_Dark.M_Red_Dark")))
          (Utilities|FlowControl|Delay 0.5)
          (if (Variables|Default|GetInLight)
            _
            (else
              (Rendering|Material|SetMaterial (Variables|Default|GetStaticMesh) 0 "/Game/SideScrollerBP/Materials/DarkWorld.DarkWorld")))
          (Utilities|FlowControl|Delay 0.5)
          (if (Variables|Default|GetInLight)
            _
            (else
              (Rendering|Material|SetMaterial (Variables|Default|GetStaticMesh) 0 "/Game/TeamFolders/Martin/Materials/M_Red_Dark.M_Red_Dark")))
          (Utilities|FlowControl|Delay 0.25)
          (if (Variables|Default|GetInLight)
            _
            (else
              (Rendering|Material|SetMaterial (Variables|Default|GetStaticMesh) 0 "/Game/SideScrollerBP/Materials/DarkWorld.DarkWorld")))
          (Utilities|FlowControl|Delay 0.25)
          (if (Variables|Default|GetInLight)
            _
            (else
              (Rendering|Material|SetMaterial (Variables|Default|GetStaticMesh) 0 "/Game/TeamFolders/Martin/Materials/M_Red_Dark.M_Red_Dark")
              (Rendering|SetVisibility (Variables|Default|GetCube) true false)
              (Variables|Default|SetLaserActive true)
              (Collision|SetCollisionEnabled (Variables|Default|GetKill%20Zone) "QueryAndPhysics")
              (Rendering|Material|SetMaterial (Variables|Default|GetCube) 0 "/Engine/VREditor/LaserPointer/LaserPointerMaterial.LaserPointerMaterial")))
          (Utilities|FlowControl|Delay 2.5)
          (Rendering|SetVisibility (Variables|Default|GetCube) false false)
          (Collision|SetCollisionEnabled (Variables|Default|GetKill%20Zone) "NoCollision")
          (Rendering|Material|SetMaterial (Variables|Default|GetStaticMesh) 0 "/Game/SideScrollerBP/Materials/DarkWorld.DarkWorld")
          (Variables|Default|SetLaserActive false)
          (goto _label))))))

(event EventBeginPlay)

(fn ConstructionScript
  (|CallParentFunction))