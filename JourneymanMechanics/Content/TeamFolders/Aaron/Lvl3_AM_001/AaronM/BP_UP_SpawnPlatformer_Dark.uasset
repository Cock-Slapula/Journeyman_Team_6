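; Spawner actor that creates dark "UP" platforms (BP_PlatformUP_Dark) at its Arrow component's location.
; On BeginPlay it spawns one platform, then calls HasSpawned on every platform of that class in the level.
; After a short delay it spawns a second platform at the same spot, with no further looping and no HasSpawned call afterwards.
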(event EventBeginPlay
  (Game|SpawnActorfromClass "/Game/TeamFolders/Aaron/Lvl3_AM_001/AaronM/BP_PlatformUP_Dark.BP_PlatformUP_Dark_C" (Math|Conversions|ToTransform(Vector) (Transformation|GetWorldLocation (Variables|Default|GetArrow))) "Undefined" 0 0)
  (Utilities|Casting|CastToBP_PlatformUP_DarkClass "/Game/TeamFolders/Aaron/Lvl3_AM_001/AaronM/BP_PlatformUP_Dark.BP_PlatformUP_Dark_C")
  (bind _outactors (Actor|GetAllActorsOfClass "/Game/TeamFolders/Aaron/Lvl3_AM_001/AaronM/BP_PlatformUP_Dark.BP_PlatformUP_Dark_C"))
  (Default|HasSpawned _outactors)
  (Utilities|FlowControl|Delay 2.0)
  (Game|SpawnActorfromClass "/Game/TeamFolders/Aaron/Lvl3_AM_001/AaronM/BP_PlatformUP_Dark.BP_PlatformUP_Dark_C" (Math|Conversions|ToTransform(Vector) (Transformation|GetWorldLocation (Variables|Default|GetArrow))) "Undefined" 0 0))

(fn ConstructionScript)