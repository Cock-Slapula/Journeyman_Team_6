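; Spike hazard Blueprint that is lethal to Mario_Character in the light world and inactive in the dark world.
; WorldWarp flips MapStateDark, running LightMode or DarkMode to swap the mesh material between laser and glass and toggle box collision and CanDie.
; Box overlap calls IsDead on the character while CanDie is set, otherwise rechecks on a short Delay loop until it is, without retesting the overlap.
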(event OnComponentBeginOverlap(Box)
  (params (OverlappedComponent :type Primitive%20Component%20Object%20Reference) (OtherActor :type Actor%20Object%20Reference) (OtherComp :type Primitive%20Component%20Object%20Reference) (OtherBodyIndex :type Integer) (bFromSweep :type Boolean) (SweepResult :type Hit%20Result%20Structure%20%28by%20ref%29))
  ;[1 1 1] Kills player on overlap
  (if (Variables|Default|GetCan%20Die) :!label _label
    (bind _asmario_character (Utilities|Casting|CastToMario_Character OtherActor))
    (Default|IsDead _asmario_character)
    (else
      (Utilities|FlowControl|Delay 0.2)
      (goto _label))))

(event Custom|World%20Warp
  ;[1 1 1] Checking which world the player is currently in and triggering the change
  (if (Variables|Default|GetMapState%20Dark)
    (CallFunction|LightMode)
    (Variables|Default|SetMapState%20Dark false)
    (else
      (CallFunction|DarkMode)
      (Variables|Default|SetMapState%20Dark true))))

(event Custom|Light%20Mode
  ;[1 1 1] Changes asset properties depending on which mode has been triggered
  (Variables|Default|SetCan%20Die true)
  (Rendering|Material|SetMaterial (Variables|Default|GetStaticMesh) 0 "/Engine/VREditor/LaserPointer/LaserPointerMaterial_Inst.LaserPointerMaterial_Inst")
  (Collision|SetCollisionEnabled (Variables|Default|GetBox) "QueryAndPhysics"))

(event Custom|Dark%20Mode
  ;[1 1 1] Changes asset properties depending on which mode has been triggered
  (Variables|Default|SetCan%20Die false)
  (Rendering|Material|SetMaterial (Variables|Default|GetStaticMesh) 0 "/Game/TeamFolders/Aaron/Lvl3_AM_001/AaronM/M_Glass.M_Glass")
  (Collision|SetCollisionEnabled (Variables|Default|GetBox) "NoCollision"))

(event EventBeginPlay
  ;[1 1 1] Sets that player can die on overlap
  (Variables|Default|SetCan%20Die true))

(fn ConstructionScript)