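; Level block that exists only in the bright world, toggling between solid and passable states when the player warps worlds.
; WorldWarp flips MapStateDark: LightMode clears the material override and enables collision, while DarkMode applies glass and disables collision.
; A Box overlap calls IsDead on Mario_Character while CanDie is set in light mode, killing a player caught inside as the block solidifies.
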(event OnComponentBeginOverlap(Box)
  (params (OverlappedComponent :type Primitive%20Component%20Object%20Reference) (OtherActor :type Actor%20Object%20Reference) (OtherComp :type Primitive%20Component%20Object%20Reference) (OtherBodyIndex :type Integer) (bFromSweep :type Boolean) (SweepResult :type Hit%20Result%20Structure%20%28by%20ref%29))
  ;[1 1 1] If player is overlapped with block mid world warp they die
  (if (Variables|Default|GetCan%20Die)
    (bind _asmario_character (Utilities|Casting|CastToMario_Character OtherActor))
    (Default|IsDead _asmario_character)))

(event Custom|World%20Warp
  ;[1 1 1] Checking which world the player is currently in and triggering the change
  (if (Variables|Default|GetMapState%20Dark)
    (CallFunction|LightMode)
    (Variables|Default|SetMapState%20Dark false)
    (else
      (CallFunction|DarkMode)
      (Variables|Default|SetMapState%20Dark true))))

(event Custom|Light%20Mode
  ;[1 1 1] Changes asset properties depending on which mode has been triggered
  (Rendering|Material|SetMaterial (Variables|Default|GetStaticMesh) 0 0)
  (Variables|Default|SetCan%20Die true)
  (Collision|SetActorEnableCollision true))

(event Custom|Dark%20Mode
  ;[1 1 1] Changes asset properties depending on which mode has been triggered
  (Rendering|Material|SetMaterial (Variables|Default|GetStaticMesh) 0 "/Game/TeamFolders/Aaron/Lvl3_AM_001/AaronM/M_Glass.M_Glass")
  (Variables|Default|SetCan%20Die false)
  (Collision|SetActorEnableCollision false))

(fn ConstructionScript)