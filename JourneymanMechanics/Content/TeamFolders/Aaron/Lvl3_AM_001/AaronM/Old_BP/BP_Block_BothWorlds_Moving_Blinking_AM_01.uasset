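; Two-world platform block that blinks, vanishes when Mario_Character touches it, and returns five seconds later.
; WorldWarp toggles LightMode and DarkMode, swapping visibility and collision between light and dark meshes according to each one's vanished state.
; Each collision overlap runs a Delay-timed material sequence, then disables collision and hides that mesh or turns it glass.
; With HasMovement set, the first overlap also starts a timeline lerping both meshes toward the Movement component's location.
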(event OnComponentBeginOverlap(LightCollision)
  (params (OverlappedComponent :type Primitive%20Component%20Object%20Reference) (OtherActor :type Actor%20Object%20Reference) (OtherComp :type Primitive%20Component%20Object%20Reference) (OtherBodyIndex :type Integer) (bFromSweep :type Boolean) (SweepResult :type Hit%20Result%20Structure%20%28by%20ref%29))
  (bind _dark_mesh (Variables|Default|GetDark%20Mesh))
  ;[1 1 1] Moving and world dissapearing system for both dark and Light Mesh
  (Utilities|Casting|CastToMario_Character OtherActor)
  (if (Variables|Default|GetHas%20Movement)
    (Variables|Default|SetDarkBox false)
    (if (Variables|Default|GetTimeline%20Undergo)
      _
      (else
        (Utilities|FlowControl|DoOnce false
          (:Completed
            (bind _newtrack_0 (Timeline|Timeline_1 Play)
              (:Update
                (Transformation|SetWorldLocation (Variables|Default|GetLight%20Mesh) (Math|Vector|Lerp(Vector) (Variables|Default|GetStart%20Coords) (Variables|Default|GetPosition%20to%20move%20to) _newtrack_0) false false)
                (Variables|Default|SetTimeline%20Undergo true)))))))
    (if (Variables|Default|GetDarkBox)
      (Rendering|Material|SetMaterial (Variables|Default|GetDark%20Mesh) 0 0)
      (Utilities|FlowControl|Delay 1.5)
      (Rendering|Material|SetMaterial (Variables|Default|GetDark%20Mesh) 0 0)
      (Utilities|FlowControl|Delay 1.5)
      (Rendering|Material|SetMaterial (Variables|Default|GetDark%20Mesh) 0 0)
      (Utilities|FlowControl|Delay 1.0)
      (Rendering|Material|SetMaterial (Variables|Default|GetDark%20Mesh) 0 0)
      (Utilities|FlowControl|Delay 0.5)
      (Rendering|Material|SetMaterial (Variables|Default|GetDark%20Mesh) 0 0)
      (Utilities|FlowControl|Delay 0.5)
      (Rendering|Material|SetMaterial (Variables|Default|GetDark%20Mesh) 0 0)
      (Utilities|FlowControl|Delay 0.5)
      (Rendering|Material|SetMaterial (Variables|Default|GetDark%20Mesh) 0 0)
      (Collision|SetCollisionEnabled _dark_mesh "NoCollision")
      (if (Variables|Default|GetHas%20Vanished%20Light)
        (Development|SetHiddeninGame _dark_mesh true false)
        (else
          (Rendering|Material|SetMaterial (Variables|Default|GetDark%20Mesh) 0 "/Game/TeamFolders/Aaron/Lvl3_AM_001/AaronM/M_Glass.M_Glass")))
      (Utilities|FlowControl|Delay 5.0)
      (Variables|Default|SetHas%20Vanished%20Dark false)
      (Effects|SpawnEmitteratLocation 0 (Transformation|GetWorldLocation (Variables|Default|GetLight%20Mesh)))
      (if (Variables|Default|GetMapState%20Dark)
        (Collision|SetCollisionEnabled (Variables|Default|GetDark%20Collision) "QueryAndPhysics")
        (Rendering|Material|SetMaterial (Variables|Default|GetDark%20Mesh) 0 0)
        (Development|SetHiddeninGame (Variables|Default|GetDark%20Collision) false false))
      (else
        (Rendering|Material|SetMaterial (Variables|Default|GetLight%20Mesh) 0 0)
        (Utilities|FlowControl|Delay 1.5)
        (Rendering|Material|SetMaterial (Variables|Default|GetLight%20Mesh) 0 0)
        (Utilities|FlowControl|Delay 1.5)
        (Rendering|Material|SetMaterial (Variables|Default|GetLight%20Mesh) 0 0)
        (Utilities|FlowControl|Delay 1.0)
        (Rendering|Material|SetMaterial (Variables|Default|GetLight%20Mesh) 0 0)
        (Utilities|FlowControl|Delay 0.5)
        (Rendering|Material|SetMaterial (Variables|Default|GetLight%20Mesh) 0 0)
        (Utilities|FlowControl|Delay 0.5)
        (Rendering|Material|SetMaterial (Variables|Default|GetLight%20Mesh) 0 0)
        (Utilities|FlowControl|Delay 0.5)
        (Rendering|Material|SetMaterial (Variables|Default|GetLight%20Mesh) 0 0)
        (Variables|Default|SetHas%20Vanished%20Light true)
        (Collision|SetCollisionEnabled (Variables|Default|GetLight%20Mesh) "NoCollision")
        (if (Variables|Default|GetHas%20Vanished%20Dark)
          (Development|SetHiddeninGame (Variables|Default|GetLight%20Mesh) true false)
          (else
            (Rendering|Material|SetMaterial (Variables|Default|GetLight%20Mesh) 0 "/Game/TeamFolders/Aaron/Lvl3_AM_001/AaronM/M_Glass.M_Glass")))
        (Utilities|FlowControl|Delay 5.0)
        (Variables|Default|SetHas%20Vanished%20Light false)
        (Effects|SpawnEmitteratLocation 0 (Transformation|GetWorldLocation (Variables|Default|GetLight%20Mesh)))
        (if (not (Variables|Default|GetMapState%20Dark))
          (Collision|SetCollisionEnabled (Variables|Default|GetLight%20Mesh) "QueryAndPhysics")
          (Rendering|Material|SetMaterial (Variables|Default|GetLight%20Mesh) 0 0)
          (Development|SetHiddeninGame (Variables|Default|GetLight%20Mesh) false false))))
    (else
      (Rendering|Material|SetMaterial (Variables|Default|GetLight%20Mesh) 0 0)
      (Utilities|FlowControl|Delay 1.0)
      (Rendering|Material|SetMaterial (Variables|Default|GetLight%20Mesh) 0 0)
      (Utilities|FlowControl|Delay 1.0)
      (Rendering|Material|SetMaterial (Variables|Default|GetLight%20Mesh) 0 0)
      (Utilities|FlowControl|Delay 0.5)
      (Rendering|Material|SetMaterial (Variables|Default|GetLight%20Mesh) 0 0)
      (Utilities|FlowControl|Delay 0.5)
      (Rendering|Material|SetMaterial (Variables|Default|GetLight%20Mesh) 0 0)
      (Utilities|FlowControl|Delay 0.5)
      (Rendering|Material|SetMaterial (Variables|Default|GetLight%20Mesh) 0 0)
      (Utilities|FlowControl|Delay 0.5)
      (Rendering|Material|SetMaterial (Variables|Default|GetLight%20Mesh) 0 0)
      (Variables|Default|SetHas%20Vanished%20Light true)
      (Collision|SetCollisionEnabled (Variables|Default|GetLight%20Mesh) "NoCollision")
      (if (Variables|Default|GetHas%20Vanished%20Dark)
        (Development|SetHiddeninGame (Variables|Default|GetLight%20Mesh) true false))
      (Rendering|Material|SetMaterial (Variables|Default|GetLight%20Mesh) 0 "/Game/TeamFolders/Aaron/Lvl3_AM_001/AaronM/M_Glass.M_Glass")
      (Utilities|FlowControl|Delay 5.0)
      (Variables|Default|SetHas%20Vanished%20Light false)
      (if (not (Variables|Default|GetMapState%20Dark))
        (Collision|SetCollisionEnabled (Variables|Default|GetLight%20Mesh) "QueryAndPhysics")
        (Rendering|Material|SetMaterial (Variables|Default|GetLight%20Mesh) 0 0)
        (Development|SetHiddeninGame (Variables|Default|GetLight%20Mesh) false false)))))

(event OnComponentBeginOverlap(DarkCollision)
  (params (OverlappedComponent :type Primitive%20Component%20Object%20Reference) (OtherActor :type Actor%20Object%20Reference) (OtherComp :type Primitive%20Component%20Object%20Reference) (OtherBodyIndex :type Integer) (bFromSweep :type Boolean) (SweepResult :type Hit%20Result%20Structure%20%28by%20ref%29))
  (bind _dark_mesh (Variables|Default|GetDark%20Mesh))
  ;[1 1 1] Moving and world dissapearing system for both dark and Light Mesh
  (Utilities|Casting|CastToMario_Character OtherActor)
  (if (Variables|Default|GetHas%20Movement)
    (Variables|Default|SetDarkBox true)
    (if (Variables|Default|GetTimeline%20Undergo)
      _
      (else
        (Utilities|FlowControl|DoOnce false
          (:Completed
            (bind _newtrack_0 (Timeline|Timeline_1 Play)
              (:Update
                (Transformation|SetWorldLocation (Variables|Default|GetLight%20Mesh) (Math|Vector|Lerp(Vector) (Variables|Default|GetStart%20Coords) (Variables|Default|GetPosition%20to%20move%20to) _newtrack_0) false false)
                (Variables|Default|SetTimeline%20Undergo true)))))))
    (if (Variables|Default|GetDarkBox)
      (Rendering|Material|SetMaterial (Variables|Default|GetDark%20Mesh) 0 0)
      (Utilities|FlowControl|Delay 1.5)
      (Rendering|Material|SetMaterial (Variables|Default|GetDark%20Mesh) 0 0)
      (Utilities|FlowControl|Delay 1.5)
      (Rendering|Material|SetMaterial (Variables|Default|GetDark%20Mesh) 0 0)
      (Utilities|FlowControl|Delay 1.0)
      (Rendering|Material|SetMaterial (Variables|Default|GetDark%20Mesh) 0 0)
      (Utilities|FlowControl|Delay 0.5)
      (Rendering|Material|SetMaterial (Variables|Default|GetDark%20Mesh) 0 0)
      (Utilities|FlowControl|Delay 0.5)
      (Rendering|Material|SetMaterial (Variables|Default|GetDark%20Mesh) 0 0)
      (Utilities|FlowControl|Delay 0.5)
      (Rendering|Material|SetMaterial (Variables|Default|GetDark%20Mesh) 0 0)
      (Collision|SetCollisionEnabled _dark_mesh "NoCollision")
      (if (Variables|Default|GetHas%20Vanished%20Light)
        (Development|SetHiddeninGame _dark_mesh true false)
        (else
          (Rendering|Material|SetMaterial (Variables|Default|GetDark%20Mesh) 0 "/Game/TeamFolders/Aaron/Lvl3_AM_001/AaronM/M_Glass.M_Glass")))
      (Utilities|FlowControl|Delay 5.0)
      (Variables|Default|SetHas%20Vanished%20Dark false)
      (Effects|SpawnEmitteratLocation 0 (Transformation|GetWorldLocation (Variables|Default|GetLight%20Mesh)))
      (if (Variables|Default|GetMapState%20Dark)
        (Collision|SetCollisionEnabled (Variables|Default|GetDark%20Collision) "QueryAndPhysics")
        (Rendering|Material|SetMaterial (Variables|Default|GetDark%20Mesh) 0 0)
        (Development|SetHiddeninGame (Variables|Default|GetDark%20Collision) false false))
      (else
        (Rendering|Material|SetMaterial (Variables|Default|GetLight%20Mesh) 0 0)
        (Utilities|FlowControl|Delay 1.5)
        (Rendering|Material|SetMaterial (Variables|Default|GetLight%20Mesh) 0 0)
        (Utilities|FlowControl|Delay 1.5)
        (Rendering|Material|SetMaterial (Variables|Default|GetLight%20Mesh) 0 0)
        (Utilities|FlowControl|Delay 1.0)
        (Rendering|Material|SetMaterial (Variables|Default|GetLight%20Mesh) 0 0)
        (Utilities|FlowControl|Delay 0.5)
        (Rendering|Material|SetMaterial (Variables|Default|GetLight%20Mesh) 0 0)
        (Utilities|FlowControl|Delay 0.5)
        (Rendering|Material|SetMaterial (Variables|Default|GetLight%20Mesh) 0 0)
        (Utilities|FlowControl|Delay 0.5)
        (Rendering|Material|SetMaterial (Variables|Default|GetLight%20Mesh) 0 0)
        (Variables|Default|SetHas%20Vanished%20Light true)
        (Collision|SetCollisionEnabled (Variables|Default|GetLight%20Mesh) "NoCollision")
        (if (Variables|Default|GetHas%20Vanished%20Dark)
          (Development|SetHiddeninGame (Variables|Default|GetLight%20Mesh) true false)
          (else
            (Rendering|Material|SetMaterial (Variables|Default|GetLight%20Mesh) 0 "/Game/TeamFolders/Aaron/Lvl3_AM_001/AaronM/M_Glass.M_Glass")))
        (Utilities|FlowControl|Delay 5.0)
        (Variables|Default|SetHas%20Vanished%20Light false)
        (Effects|SpawnEmitteratLocation 0 (Transformation|GetWorldLocation (Variables|Default|GetLight%20Mesh)))
        (if (not (Variables|Default|GetMapState%20Dark))
          (Collision|SetCollisionEnabled (Variables|Default|GetLight%20Mesh) "QueryAndPhysics")
          (Rendering|Material|SetMaterial (Variables|Default|GetLight%20Mesh) 0 0)
          (Development|SetHiddeninGame (Variables|Default|GetLight%20Mesh) false false))))
    (else
      (Rendering|Material|SetMaterial (Variables|Default|GetDark%20Mesh) 0 0)
      (Utilities|FlowControl|Delay 1.0)
      (Rendering|Material|SetMaterial (Variables|Default|GetDark%20Mesh) 0 0)
      (Utilities|FlowControl|Delay 1.0)
      (Rendering|Material|SetMaterial (Variables|Default|GetDark%20Mesh) 0 0)
      (Utilities|FlowControl|Delay 0.5)
      (Rendering|Material|SetMaterial (Variables|Default|GetDark%20Mesh) 0 0)
      (Utilities|FlowControl|Delay 0.5)
      (Rendering|Material|SetMaterial (Variables|Default|GetDark%20Mesh) 0 0)
      (Utilities|FlowControl|Delay 0.5)
      (Rendering|Material|SetMaterial (Variables|Default|GetDark%20Mesh) 0 0)
      (Utilities|FlowControl|Delay 0.5)
      (Rendering|Material|SetMaterial (Variables|Default|GetDark%20Mesh) 0 0)
      (Variables|Default|SetHas%20Vanished%20Dark true)
      (Collision|SetCollisionEnabled (Variables|Default|GetDark%20Mesh) "NoCollision")
      (if (Variables|Default|GetHas%20Vanished%20Light)
        (Development|SetHiddeninGame (Variables|Default|GetDark%20Collision) true false)
        (else
          (Rendering|Material|SetMaterial (Variables|Default|GetDark%20Mesh) 0 "/Game/TeamFolders/Aaron/Lvl3_AM_001/AaronM/M_Glass.M_Glass")))
      (Utilities|FlowControl|Delay 5.0)
      (Variables|Default|SetHas%20Vanished%20Dark false)
      (if (Variables|Default|GetMapState%20Dark)
        (Collision|SetCollisionEnabled (Variables|Default|GetDark%20Mesh) "QueryAndPhysics")
        (Rendering|Material|SetMaterial (Variables|Default|GetDark%20Mesh) 0 0)
        (Development|SetHiddeninGame (Variables|Default|GetDark%20Mesh) false false)))))

(event Custom|World%20Warp
  ;[1 1 1] Checking which world the player is currently in and triggering the change
  (if (Variables|Default|GetMapState%20Dark)
    (CallFunction|LightMode)
    (Variables|Default|SetMapState%20Dark false)
    (else
      (CallFunction|DarkMode)
      (Variables|Default|SetMapState%20Dark true))))

(event Custom|Light%20Mode
  ;[1 1 1] Checking which world the player is currently in and triggering the changes depending if one or more collision boxes have been overlapped
  (Variables|Default|SetMapState%20Dark false)
  (if (Variables|Default|GetHas%20Vanished%20Light)
    (Development|SetHiddeninGame (Variables|Default|GetLight%20Mesh) true false)
    (Collision|SetCollisionEnabled (Variables|Default|GetLight%20Mesh) "NoCollision")
    (Collision|SetCollisionEnabled (Variables|Default|GetDark%20Collision) "NoCollision")
    (Rendering|Material|SetMaterial (Variables|Default|GetDark%20Mesh) 0 "/Game/TeamFolders/Aaron/Lvl3_AM_001/AaronM/M_Glass.M_Glass")
    (else
      (Rendering|Material|SetMaterial (Variables|Default|GetLight%20Mesh) 0 0)
      (Collision|SetCollisionEnabled (Variables|Default|GetLight%20Collision) "QueryAndPhysics")
      (Development|SetHiddeninGame (Variables|Default|GetLight%20Mesh) false false)
      (Development|SetHiddeninGame (Variables|Default|GetDark%20Mesh) true false)
      (Collision|SetCollisionEnabled (Variables|Default|GetDark%20Mesh) "NoCollision"))))

(event Custom|Dark%20Mode
  ;[1 1 1] Checking which world the player is currently in and triggering the changes depending if one or more collision boxes have been overlapped
  (Variables|Default|SetMapState%20Dark true)
  (if (Variables|Default|GetHas%20Vanished%20Dark)
    (Development|SetHiddeninGame (Variables|Default|GetLight%20Mesh) true false)
    (Development|SetHiddeninGame (Variables|Default|GetDark%20Mesh) false false)
    (Collision|SetCollisionEnabled (Variables|Default|GetDark%20Mesh) "NoCollision")
    (Collision|SetCollisionEnabled (Variables|Default|GetLight%20Mesh) "NoCollision")
    (Rendering|Material|SetMaterial (Variables|Default|GetLight%20Mesh) 0 "/Game/TeamFolders/Aaron/Lvl3_AM_001/AaronM/M_Glass.M_Glass")
    (else
      (Rendering|Material|SetMaterial (Variables|Default|GetDark%20Mesh) 0 0)
      (Collision|SetCollisionEnabled (Variables|Default|GetDark%20Mesh) "QueryAndPhysics")
      (Collision|SetCollisionEnabled (Variables|Default|GetLight%20Mesh) "NoCollision")
      (Development|SetHiddeninGame (Variables|Default|GetLight%20Mesh) true false)
      (Development|SetHiddeninGame (Variables|Default|GetDark%20Mesh) false false))))

(event EventBeginPlay
  (bind _light_mesh (Variables|Default|GetLight%20Mesh))
  (bind _relativelocation (Variables|/Script/Engine.SceneComponent|GetRelativeLocation _light_mesh))
  ;[1 1 1] Gets Coords if moving and sets the dark meshs collision to none
  (Variables|Default|SetPosition%20to%20move%20to (Transformation|GetWorldLocation (Variables|Default|GetMovement)))
  (Variables|Default|SetStart%20Coords (Transformation|GetWorldLocation (Variables|Default|GetLight%20Mesh)))
  (Variables|Default|SetY (.y _relativelocation))
  (Variables|Default|SetZ (.z _relativelocation))
  (Collision|SetCollisionEnabled (Variables|Default|GetDark%20Collision) "NoCollision")
  (Development|SetHiddeninGame (Variables|Default|GetDark%20Mesh) true false)
  (Rendering|Material|SetMaterial (Variables|Default|GetDark%20Mesh) 0 "/Game/TeamFolders/Aaron/Lvl3_AM_001/AaronM/M_Glass.M_Glass"))

(fn ConstructionScript)