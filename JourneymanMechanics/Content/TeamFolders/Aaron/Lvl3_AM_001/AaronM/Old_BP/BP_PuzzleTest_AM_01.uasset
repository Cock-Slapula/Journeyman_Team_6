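; Light/dark puzzle actor with seven blocks that opens a locked door once all are locked.
; WorldWarp toggles map state, moving each block between two X offsets and resetting its material according to its Bright/Dark flag.
; Mario_Character overlaps on block triggers set that flag and lock from the current state, then UnlockDoor opens the first BP_LockedDoor_AM_01 when all locks are true.
; Other boxes call IsDead on the character.
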(event OnComponentBeginOverlap(Box)
  (params (OverlappedComponent :type Primitive%20Component%20Object%20Reference) (OtherActor :type Actor%20Object%20Reference) (OtherComp :type Primitive%20Component%20Object%20Reference) (OtherBodyIndex :type Integer) (bFromSweep :type Boolean) (SweepResult :type Hit%20Result%20Structure%20%28by%20ref%29))
  (bind _block_1 (Variables|Default|GetBlock_1))
  (Utilities|Casting|CastToMario_Character OtherActor)
  (if (Variables|Default|GetMap_State_Dark)
    (Variables|Default|SetBlock1%20%28Bright%29 true)
    (Variables|Default|SetBloc1%20LOCK true)
    (else
      (Variables|Default|SetBlock1%20%28Bright%29 false)
      (Variables|Default|SetBloc1%20LOCK false)))
  (Transformation|SetRelativeLocation _block_1 (Math|Vector|MakeVector -25.0 (Variables|Default|GetBlock1%20Y) (Variables|Default|GetBlock1%20Z)) false false)
  (Rendering|Material|SetMaterial _block_1 0 0)
  (CallFunction|UnlockDoor))

(event OnComponentBeginOverlap(Box1)
  (params (OverlappedComponent :type Primitive%20Component%20Object%20Reference) (OtherActor :type Actor%20Object%20Reference) (OtherComp :type Primitive%20Component%20Object%20Reference) (OtherBodyIndex :type Integer) (bFromSweep :type Boolean) (SweepResult :type Hit%20Result%20Structure%20%28by%20ref%29))
  (bind _block_2 (Variables|Default|GetBlock_2))
  (Utilities|Casting|CastToMario_Character OtherActor)
  (if (Variables|Default|GetMap_State_Dark)
    (Variables|Default|SetBlock2%20%28Dark%29 true)
    (Variables|Default|SetBloc2%20LOCK false)
    (else
      (Variables|Default|SetBlock2%20%28Dark%29 false)
      (Variables|Default|SetBloc2%20LOCK true)))
  (Transformation|SetRelativeLocation _block_2 (Math|Vector|MakeVector -25.0 (Variables|Default|GetBlock2%20Y) (Variables|Default|GetBlock2%20Z)) false false)
  (Rendering|Material|SetMaterial _block_2 0 0)
  (CallFunction|UnlockDoor))

(event OnComponentBeginOverlap(Box10)
  (params (OverlappedComponent :type Primitive%20Component%20Object%20Reference) (OtherActor :type Actor%20Object%20Reference) (OtherComp :type Primitive%20Component%20Object%20Reference) (OtherBodyIndex :type Integer) (bFromSweep :type Boolean) (SweepResult :type Hit%20Result%20Structure%20%28by%20ref%29))
  (bind _asmario_character (Utilities|Casting|CastToMario_Character OtherActor))
  (Default|IsDead _asmario_character))

(event OnComponentBeginOverlap(Box11)
  (params (OverlappedComponent :type Primitive%20Component%20Object%20Reference) (OtherActor :type Actor%20Object%20Reference) (OtherComp :type Primitive%20Component%20Object%20Reference) (OtherBodyIndex :type Integer) (bFromSweep :type Boolean) (SweepResult :type Hit%20Result%20Structure%20%28by%20ref%29))
  (bind _asmario_character (Utilities|Casting|CastToMario_Character OtherActor))
  (Default|IsDead _asmario_character))

(event OnComponentBeginOverlap(Box14)
  (params (OverlappedComponent :type Primitive%20Component%20Object%20Reference) (OtherActor :type Actor%20Object%20Reference) (OtherComp :type Primitive%20Component%20Object%20Reference) (OtherBodyIndex :type Integer) (bFromSweep :type Boolean) (SweepResult :type Hit%20Result%20Structure%20%28by%20ref%29))
  (bind _asmario_character (Utilities|Casting|CastToMario_Character OtherActor))
  (Default|IsDead _asmario_character))

(event OnComponentBeginOverlap(Box18)
  (params (OverlappedComponent :type Primitive%20Component%20Object%20Reference) (OtherActor :type Actor%20Object%20Reference) (OtherComp :type Primitive%20Component%20Object%20Reference) (OtherBodyIndex :type Integer) (bFromSweep :type Boolean) (SweepResult :type Hit%20Result%20Structure%20%28by%20ref%29))
  (bind _asmario_character (Utilities|Casting|CastToMario_Character OtherActor))
  (Default|IsDead _asmario_character))

(event OnComponentBeginOverlap(Box2)
  (params (OverlappedComponent :type Primitive%20Component%20Object%20Reference) (OtherActor :type Actor%20Object%20Reference) (OtherComp :type Primitive%20Component%20Object%20Reference) (OtherBodyIndex :type Integer) (bFromSweep :type Boolean) (SweepResult :type Hit%20Result%20Structure%20%28by%20ref%29))
  (bind _block_3 (Variables|Default|GetBlock_3))
  (Utilities|Casting|CastToMario_Character OtherActor)
  (if (Variables|Default|GetMap_State_Dark)
    (Variables|Default|SetBlock3%20%28Bright%29 true)
    (Variables|Default|SetBloc3%20LOCK true)
    (else
      (Variables|Default|SetBlock3%20%28Bright%29 false)
      (Variables|Default|SetBloc3%20LOCK false)))
  (Transformation|SetRelativeLocation _block_3 (Math|Vector|MakeVector -25.0 (Variables|Default|GetBlock3%20Y) (Variables|Default|GetBlock3%20Z)) false false)
  (Rendering|Material|SetMaterial _block_3 0 0)
  (CallFunction|UnlockDoor))

(event OnComponentBeginOverlap(Box12)
  (params (OverlappedComponent :type Primitive%20Component%20Object%20Reference) (OtherActor :type Actor%20Object%20Reference) (OtherComp :type Primitive%20Component%20Object%20Reference) (OtherBodyIndex :type Integer) (bFromSweep :type Boolean) (SweepResult :type Hit%20Result%20Structure%20%28by%20ref%29))
  (bind _asmario_character (Utilities|Casting|CastToMario_Character OtherActor))
  (Default|IsDead _asmario_character))

(event OnComponentBeginOverlap(BoxA)
  (params (OverlappedComponent :type Primitive%20Component%20Object%20Reference) (OtherActor :type Actor%20Object%20Reference) (OtherComp :type Primitive%20Component%20Object%20Reference) (OtherBodyIndex :type Integer) (bFromSweep :type Boolean) (SweepResult :type Hit%20Result%20Structure%20%28by%20ref%29))
  (bind _asmario_character (Utilities|Casting|CastToMario_Character OtherActor))
  (Default|IsDead _asmario_character))

(event OnComponentBeginOverlap(Box3)
  (params (OverlappedComponent :type Primitive%20Component%20Object%20Reference) (OtherActor :type Actor%20Object%20Reference) (OtherComp :type Primitive%20Component%20Object%20Reference) (OtherBodyIndex :type Integer) (bFromSweep :type Boolean) (SweepResult :type Hit%20Result%20Structure%20%28by%20ref%29))
  (bind _block_4 (Variables|Default|GetBlock_4))
  (Utilities|Casting|CastToMario_Character OtherActor)
  (Audio|PlaySound2D 0 1.0 1.0 0.0 0 0)
  (if (Variables|Default|GetMap_State_Dark)
    (Variables|Default|SetBlock4%20%28Dark%29 true)
    (Variables|Default|SetBloc4%20LOCK false)
    (else
      (Variables|Default|SetBlock4%20%28Dark%29 false)
      (Variables|Default|SetBloc4%20LOCK true)))
  (Transformation|SetRelativeLocation _block_4 (Math|Vector|MakeVector -25.0 (Variables|Default|GetBloack4_Y) (Variables|Default|GetBlock4_Z)) false false)
  (Rendering|Material|SetMaterial _block_4 0 0)
  (CallFunction|UnlockDoor))

(event OnComponentBeginOverlap(Box4)
  (params (OverlappedComponent :type Primitive%20Component%20Object%20Reference) (OtherActor :type Actor%20Object%20Reference) (OtherComp :type Primitive%20Component%20Object%20Reference) (OtherBodyIndex :type Integer) (bFromSweep :type Boolean) (SweepResult :type Hit%20Result%20Structure%20%28by%20ref%29))
  (bind _block_5 (Variables|Default|GetBlock_5))
  (Utilities|Casting|CastToMario_Character OtherActor)
  (if (Variables|Default|GetMap_State_Dark)
    (Variables|Default|SetBlock5%20%28Bright%29 false)
    (Variables|Default|SetBloc5%20LOCK true)
    (else
      (Variables|Default|SetBlock5%20%28Bright%29 true)
      (Variables|Default|SetBloc5%20LOCK false)))
  (Transformation|SetRelativeLocation _block_5 (Math|Vector|MakeVector -25.0 (Variables|Default|GetBlock5%20Y) (Variables|Default|GetBlock5%20Z)) false false)
  (Rendering|Material|SetMaterial _block_5 0 0)
  (CallFunction|UnlockDoor))

(event OnComponentBeginOverlap(Box5)
  (params (OverlappedComponent :type Primitive%20Component%20Object%20Reference) (OtherActor :type Actor%20Object%20Reference) (OtherComp :type Primitive%20Component%20Object%20Reference) (OtherBodyIndex :type Integer) (bFromSweep :type Boolean) (SweepResult :type Hit%20Result%20Structure%20%28by%20ref%29))
  (bind _block_6 (Variables|Default|GetBlock_6))
  (Utilities|Casting|CastToMario_Character OtherActor)
  (if (Variables|Default|GetMap_State_Dark)
    (Variables|Default|SetBlock6%20%28Dark%29 false)
    (Variables|Default|SetBloc6%20LOCK false)
    (else
      (Variables|Default|SetBlock6%20%28Dark%29 true)
      (Variables|Default|SetBloc6%20LOCK true)))
  (Transformation|SetRelativeLocation _block_6 (Math|Vector|MakeVector -25.0 (Variables|Default|GetBlock6%20Y) (Variables|Default|GetBlock6%20Z)) false false)
  (Rendering|Material|SetMaterial _block_6 0 0)
  (CallFunction|UnlockDoor))

(event OnComponentBeginOverlap(Box6)
  (params (OverlappedComponent :type Primitive%20Component%20Object%20Reference) (OtherActor :type Actor%20Object%20Reference) (OtherComp :type Primitive%20Component%20Object%20Reference) (OtherBodyIndex :type Integer) (bFromSweep :type Boolean) (SweepResult :type Hit%20Result%20Structure%20%28by%20ref%29))
  (bind _block_7 (Variables|Default|GetBlock_7))
  (Utilities|Casting|CastToMario_Character OtherActor)
  (if (Variables|Default|GetMap_State_Dark)
    (Variables|Default|SetBlock7%20%28Bright%29 false)
    (Variables|Default|SetBloc7%20LOCK true)
    (else
      (Variables|Default|SetBlock7%20%28Bright%29 true)
      (Variables|Default|SetBloc7%20LOCK false)))
  (Transformation|SetRelativeLocation _block_7 (Math|Vector|MakeVector -25.0 (Variables|Default|GetBlock7%20Y) (Variables|Default|GetBlock7%20Z)) false false)
  (Rendering|Material|SetMaterial _block_7 0 0)
  (CallFunction|UnlockDoor))

(event OnComponentBeginOverlap(Box8)
  (params (OverlappedComponent :type Primitive%20Component%20Object%20Reference) (OtherActor :type Actor%20Object%20Reference) (OtherComp :type Primitive%20Component%20Object%20Reference) (OtherBodyIndex :type Integer) (bFromSweep :type Boolean) (SweepResult :type Hit%20Result%20Structure%20%28by%20ref%29))
  (bind _asmario_character (Utilities|Casting|CastToMario_Character OtherActor))
  (Default|IsDead _asmario_character))

(event OnComponentBeginOverlap(Box9)
  (params (OverlappedComponent :type Primitive%20Component%20Object%20Reference) (OtherActor :type Actor%20Object%20Reference) (OtherComp :type Primitive%20Component%20Object%20Reference) (OtherBodyIndex :type Integer) (bFromSweep :type Boolean) (SweepResult :type Hit%20Result%20Structure%20%28by%20ref%29))
  (bind _asmario_character (Utilities|Casting|CastToMario_Character OtherActor))
  (Default|IsDead _asmario_character))

(event Custom|World%20Warp
  ;[1 1 1] The Brain
  (if (Variables|Default|GetMap_State_Dark)
    (CallFunction|LightMode)
    (else
      (CallFunction|DarkMode))))

(event Custom|Light%20Mode
  (bind _block1_y (Variables|Default|GetBlock1%20Y))
  (bind _block1_z (Variables|Default|GetBlock1%20Z))
  (bind _block_5 (Variables|Default|GetBlock_5))
  (bind _block2_z (Variables|Default|GetBlock2%20Z))
  (bind _block2_y (Variables|Default|GetBlock2%20Y))
  (bind _block_2 (Variables|Default|GetBlock_2))
  (bind _block5_y (Variables|Default|GetBlock5%20Y))
  (bind _block3_z (Variables|Default|GetBlock3%20Z))
  (bind _block3_y (Variables|Default|GetBlock3%20Y))
  (bind _block_3 (Variables|Default|GetBlock_3))
  (bind _block5_z (Variables|Default|GetBlock5%20Z))
  (bind _block_4 (Variables|Default|GetBlock_4))
  (bind _block4_z (Variables|Default|GetBlock4_Z))
  (bind _bloack4_y (Variables|Default|GetBloack4_Y))
  (bind _block_6 (Variables|Default|GetBlock_6))
  (bind _block6_y (Variables|Default|GetBlock6%20Y))
  (bind _block6_z (Variables|Default|GetBlock6%20Z))
  (bind _block7_y (Variables|Default|GetBlock7%20Y))
  (bind _block7_z (Variables|Default|GetBlock7%20Z))
  (bind _block_7 (Variables|Default|GetBlock_7))
  (bind _block_1 (Variables|Default|GetBlock_1))
  (Variables|Default|SetMap_State_Dark false)
  (if (Variables|Default|GetBlock1%20%28Bright%29)
    (Transformation|SetRelativeLocation _block_1 (Math|Vector|MakeVector 25.0 _block1_y _block1_z) false false)
    (Rendering|Material|SetMaterial _block_1 0 0)
    (else
      (Transformation|SetRelativeLocation _block_1 (Math|Vector|MakeVector -25.0 _block1_y _block1_z) false false)
      (Rendering|Material|SetMaterial _block_1 0 0)))
  (if (Variables|Default|GetBlock2%20%28Dark%29)
    (Transformation|SetRelativeLocation _block_2 (Math|Vector|MakeVector 25.0 _block2_y _block2_z) false false)
    (Rendering|Material|SetMaterial _block_2 0 0)
    (else
      (Transformation|SetRelativeLocation _block_2 (Math|Vector|MakeVector -25.0 _block2_y _block2_z) false false)
      (Rendering|Material|SetMaterial _block_2 0 0)))
  (if (Variables|Default|GetBlock3%20%28Bright%29)
    (Transformation|SetRelativeLocation _block_3 (Math|Vector|MakeVector 25.0 _block3_y _block3_z) false false)
    (Rendering|Material|SetMaterial _block_3 0 0)
    (else
      (Transformation|SetRelativeLocation _block_3 (Math|Vector|MakeVector -25.0 _block3_y _block3_z) false false)
      (Rendering|Material|SetMaterial _block_3 0 0)))
  (if (Variables|Default|GetBlock4%20%28Dark%29)
    (Transformation|SetRelativeLocation _block_4 (Math|Vector|MakeVector 25.0 _bloack4_y _block4_z) false false)
    (Rendering|Material|SetMaterial _block_4 0 0)
    (else
      (Transformation|SetRelativeLocation _block_4 (Math|Vector|MakeVector -25.0 _bloack4_y _block4_z) false false)
      (Rendering|Material|SetMaterial _block_4 0 0)))
  (if (Variables|Default|GetBlock5%20%28Bright%29)
    (Transformation|SetRelativeLocation _block_5 (Math|Vector|MakeVector -25.0 _block5_y _block5_z) false false)
    (Rendering|Material|SetMaterial _block_5 0 0)
    (else
      (Transformation|SetRelativeLocation _block_5 (Math|Vector|MakeVector 25.0 _block5_y _block5_z) false false)
      (Rendering|Material|SetMaterial _block_5 0 0)))
  (if (Variables|Default|GetBlock6%20%28Dark%29)
    (Transformation|SetRelativeLocation _block_6 (Math|Vector|MakeVector -25.0 _block6_y _block6_z) false false)
    (Rendering|Material|SetMaterial _block_6 0 0)
    (else
      (Transformation|SetRelativeLocation _block_6 (Math|Vector|MakeVector 25.0 _block6_y _block6_z) false false)
      (Rendering|Material|SetMaterial _block_6 0 0)))
  (if (Variables|Default|GetBlock7%20%28Bright%29)
    (Transformation|SetRelativeLocation _block_7 (Math|Vector|MakeVector -25.0 _block7_y _block7_z) false false)
    (Rendering|Material|SetMaterial _block_7 0 0)
    (else
      (Transformation|SetRelativeLocation _block_7 (Math|Vector|MakeVector 25.0 _block7_y _block7_z) false false)
      (Rendering|Material|SetMaterial _block_7 0 0))))

(event Custom|Dark%20Mode
  (bind _block1_y (Variables|Default|GetBlock1%20Y))
  (bind _block1_z (Variables|Default|GetBlock1%20Z))
  (bind _block_5 (Variables|Default|GetBlock_5))
  (bind _block2_z (Variables|Default|GetBlock2%20Z))
  (bind _block2_y (Variables|Default|GetBlock2%20Y))
  (bind _block_2 (Variables|Default|GetBlock_2))
  (bind _block5_y (Variables|Default|GetBlock5%20Y))
  (bind _block3_z (Variables|Default|GetBlock3%20Z))
  (bind _block3_y (Variables|Default|GetBlock3%20Y))
  (bind _block_3 (Variables|Default|GetBlock_3))
  (bind _block5_z (Variables|Default|GetBlock5%20Z))
  (bind _block_4 (Variables|Default|GetBlock_4))
  (bind _block4_z (Variables|Default|GetBlock4_Z))
  (bind _bloack4_y (Variables|Default|GetBloack4_Y))
  (bind _block_6 (Variables|Default|GetBlock_6))
  (bind _block6_y (Variables|Default|GetBlock6%20Y))
  (bind _block6_z (Variables|Default|GetBlock6%20Z))
  (bind _block7_y (Variables|Default|GetBlock7%20Y))
  (bind _block7_z (Variables|Default|GetBlock7%20Z))
  (bind _block_7 (Variables|Default|GetBlock_7))
  (bind _block_1 (Variables|Default|GetBlock_1))
  (Variables|Default|SetMap_State_Dark true)
  (if (Variables|Default|GetBlock1%20%28Bright%29)
    (Transformation|SetRelativeLocation _block_1 (Math|Vector|MakeVector -25.0 _block1_y _block1_z) false false)
    (Rendering|Material|SetMaterial _block_1 0 0)
    (else
      (Transformation|SetRelativeLocation _block_1 (Math|Vector|MakeVector 25.0 _block1_y _block1_z) false false)
      (Rendering|Material|SetMaterial _block_1 0 0)))
  (if (Variables|Default|GetBlock2%20%28Dark%29)
    (Transformation|SetRelativeLocation _block_2 (Math|Vector|MakeVector -25.0 _block2_y _block2_z) false false)
    (Rendering|Material|SetMaterial _block_2 0 0)
    (else
      (Transformation|SetRelativeLocation _block_2 (Math|Vector|MakeVector 25.0 _block2_y _block2_z) false false)
      (Rendering|Material|SetMaterial _block_2 0 0)))
  (if (Variables|Default|GetBlock3%20%28Bright%29)
    (Transformation|SetRelativeLocation _block_3 (Math|Vector|MakeVector -25.0 _block3_y _block3_z) false false)
    (Rendering|Material|SetMaterial _block_3 0 0)
    (else
      (Transformation|SetRelativeLocation _block_3 (Math|Vector|MakeVector 25.0 _block3_y _block3_z) false false)
      (Rendering|Material|SetMaterial _block_3 0 0)))
  (if (Variables|Default|GetBlock4%20%28Dark%29)
    (Transformation|SetRelativeLocation _block_4 (Math|Vector|MakeVector -25.0 _bloack4_y _block4_z) false false)
    (Rendering|Material|SetMaterial _block_4 0 0)
    (else
      (Transformation|SetRelativeLocation _block_4 (Math|Vector|MakeVector 25.0 _bloack4_y _block4_z) false false)
      (Rendering|Material|SetMaterial _block_4 0 0)))
  (if (Variables|Default|GetBlock5%20%28Bright%29)
    (Transformation|SetRelativeLocation _block_5 (Math|Vector|MakeVector 25.0 _block5_y _block5_z) false false)
    (Rendering|Material|SetMaterial _block_5 0 0)
    (else
      (Transformation|SetRelativeLocation _block_5 (Math|Vector|MakeVector -25.0 _block5_y _block5_z) false false)
      (Rendering|Material|SetMaterial _block_5 0 0)))
  (if (Variables|Default|GetBlock6%20%28Dark%29)
    (Transformation|SetRelativeLocation _block_6 (Math|Vector|MakeVector 25.0 _block6_y _block6_z) false false)
    (Rendering|Material|SetMaterial _block_6 0 0)
    (else
      (Transformation|SetRelativeLocation _block_6 (Math|Vector|MakeVector -25.0 _block6_y _block6_z) false false)
      (Rendering|Material|SetMaterial _block_6 0 0)))
  (if (Variables|Default|GetBlock7%20%28Bright%29)
    (Transformation|SetRelativeLocation _block_7 (Math|Vector|MakeVector 25.0 _block7_y _block7_z) false false)
    (Rendering|Material|SetMaterial _block_7 0 0)
    (else
      (Transformation|SetRelativeLocation _block_7 (Math|Vector|MakeVector -25.0 _block7_y _block7_z) false false)
      (Rendering|Material|SetMaterial _block_7 0 0))))

(event Custom|Unlock%20Door
  (if (Variables|Default|GetBloc1%20LOCK)
    (if (Variables|Default|GetBloc2%20LOCK)
      (if (Variables|Default|GetBloc3%20LOCK)
        (if (Variables|Default|GetBloc4%20LOCK)
          (if (Variables|Default|GetBloc5%20LOCK)
            (if (Variables|Default|GetBloc6%20LOCK)
              (if (Variables|Default|GetBloc7%20LOCK)
                (bind _outactors (Actor|GetAllActorsOfClass "/Game/TeamFolders/Aaron/Lvl3_AM_001/AaronM/Old_BP/BP_LockedDoor_AM_01.BP_LockedDoor_AM_01_C"))
                (bind _asbp_locked_door_am_01 (Utilities|Casting|CastToBP_LockedDoor_AM_01 (Utilities|Array|Get(acopy) _outactors)))
                (Default|Open _asbp_locked_door_am_01)))))))))

(event EventBeginPlay
  (bind _block_1 (Variables|Default|GetBlock_1))
  (bind _block_2 (Variables|Default|GetBlock_2))
  (bind _block_3 (Variables|Default|GetBlock_3))
  (bind _block_4 (Variables|Default|GetBlock_4))
  (bind _block_5 (Variables|Default|GetBlock_5))
  (bind _block_6 (Variables|Default|GetBlock_6))
  (bind _block_7 (Variables|Default|GetBlock_7))
  (bind _relativelocation (Variables|/Script/Engine.SceneComponent|GetRelativeLocation _block_1))
  (bind _relativelocation_2 (Variables|/Script/Engine.SceneComponent|GetRelativeLocation _block_2))
  (bind _relativelocation_3 (Variables|/Script/Engine.SceneComponent|GetRelativeLocation _block_3))
  (bind _relativelocation_4 (Variables|/Script/Engine.SceneComponent|GetRelativeLocation _block_4))
  (bind _relativelocation_5 (Variables|/Script/Engine.SceneComponent|GetRelativeLocation _block_5))
  (bind _relativelocation_6 (Variables|/Script/Engine.SceneComponent|GetRelativeLocation _block_6))
  (bind _relativelocation_7 (Variables|/Script/Engine.SceneComponent|GetRelativeLocation _block_7))
  (Variables|Default|SetBlock1%20Y (.y _relativelocation))
  (Variables|Default|SetBlock1%20Z (.z _relativelocation))
  (Variables|Default|SetBlock2%20Y (.y _relativelocation_2))
  (Variables|Default|SetBlock2%20Z (.z _relativelocation_2))
  (Variables|Default|SetBlock3%20Y (.y _relativelocation_3))
  (Variables|Default|SetBlock3%20Z (.z _relativelocation_3))
  (Variables|Default|SetBloack4_Y (.y _relativelocation_4))
  (Variables|Default|SetBlock4_Z (.z _relativelocation_4))
  (Variables|Default|SetBlock5%20Y (.y _relativelocation_5))
  (Variables|Default|SetBlock5%20Z (.z _relativelocation_5))
  (Variables|Default|SetBlock6%20Z (.z _relativelocation_6))
  (Variables|Default|SetBlock6%20Y (.y _relativelocation_6))
  (Variables|Default|SetBlock7%20Y (.y _relativelocation_7))
  (Variables|Default|SetBlock7%20Z (.z _relativelocation_7)))

(event Collision|EventActorBeginOverlap
  (params (OtherActor :type Actor%20Object%20Reference)))

(event EventTick
  (params (DeltaSeconds :type Float%20%28single-precision%29)))

(fn ConstructionScript)