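; A dark-world platform block that either moves or falls when Mario_Character enters its trigger.
; WorldWarp toggles it between a glass, non-colliding light state and a solid dark state, in which overlapping its kill box calls IsDead on the player.
; Depending on the Drop flag, timelines lerp the mesh to a movement point, or after a delay to a drop point where it loses collision and hides.
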(event OnComponentBeginOverlap(Box)
  (params (OverlappedComponent :type Primitive%20Component%20Object%20Reference) (OtherActor :type Actor%20Object%20Reference) (OtherComp :type Primitive%20Component%20Object%20Reference) (OtherBodyIndex :type Integer) (bFromSweep :type Boolean) (SweepResult :type Hit%20Result%20Structure%20%28by%20ref%29))
  ;[1 1 1] Player can die if overlapped with the hitbox mid world warp
  (if (Variables|Default|GetCan%20Die)
    (bind _asmario_character (Utilities|Casting|CastToMario_Character OtherActor))
    (Default|IsDead _asmario_character)))

(event OnComponentBeginOverlap(Box1)
  (params (OverlappedComponent :type Primitive%20Component%20Object%20Reference) (OtherActor :type Actor%20Object%20Reference) (OtherComp :type Primitive%20Component%20Object%20Reference) (OtherBodyIndex :type Integer) (bFromSweep :type Boolean) (SweepResult :type Hit%20Result%20Structure%20%28by%20ref%29))
  ;[1 1 1] Movement/Drop
  (Utilities|Casting|CastToMario_Character OtherActor)
  (if (Variables|Default|GetDrop)
    (Rendering|Material|SetMaterial (Variables|Default|GetStaticMesh) 0 0)
    (Utilities|FlowControl|Delay (Variables|Default|GetTime))
    (bind _newtrack_0 (Timeline|Timeline_1 Play)
      (:Update
        (Transformation|SetWorldLocation (Variables|Default|GetStaticMesh) (Math|Vector|Lerp(Vector) (Variables|Default|GetStart%20Loc) (Variables|Default|GetDrop%20Box%20Loc) _newtrack_0) false false)
        (Utilities|FlowControl|Delay 0.4)
        (Collision|SetCollisionEnabled (Variables|Default|GetStaticMesh) "NoCollision")
        (Development|SetHiddeninGame (Variables|Default|GetStaticMesh) true false)))
    (else
      (bind _newtrack_0_2 (Timeline|Timeline_0 Play)
        (:Update
          (Transformation|SetWorldLocation (Variables|Default|GetStaticMesh) (Math|Vector|Lerp(Vector) (Variables|Default|GetStart%20Loc) (Variables|Default|GetEnd%20Loc) _newtrack_0_2) false false))))))

(event Custom|World%20Warp
  ;[1 1 1] Checking which world the player is currently in and triggering the change
  (if (Variables|Default|GetMapState%20Dark)
    (CallFunction|LightMode)
    (Variables|Default|SetMapState%20Dark false)
    (else
      (CallFunction|DarkMode)
      (Variables|Default|SetMapState%20Dark true))))

(event Custom|Light%20Mode
  ;[1 1 1] Changes asset properties depending on which mode has been triggered
  (Rendering|Material|SetMaterial (Variables|Default|GetStaticMesh) 0 "/Game/TeamFolders/Aaron/Lvl3_AM_001/AaronM/M_Glass.M_Glass")
  (Variables|Default|SetCan%20Die false)
  ;[1 1 1] Gets Coords and sets collision to none
  (Collision|SetCollisionEnabled (Variables|Default|GetBox1) "NoCollision"))

(event Custom|Dark%20Mode
  ;[1 1 1] Changes asset properties depending on which mode has been triggered
  (Rendering|Material|SetMaterial (Variables|Default|GetStaticMesh) 0 0)
  (Variables|Default|SetCan%20Die true)
  (Collision|SetCollisionEnabled (Variables|Default|GetBox1) "QueryAndPhysics"))

(event EventBeginPlay
  ;[1 1 1] Gets Coords and sets collision to none
  (Variables|Default|SetStart%20Loc (Transformation|GetWorldLocation (Variables|Default|GetStaticMesh)))
  (Variables|Default|SetEnd%20Loc (Transformation|GetWorldLocation (Variables|Default|GetMovement)))
  (Variables|Default|SetDrop%20Box%20Loc (Transformation|GetWorldLocation (Variables|Default|GetDrobBox)))
  (Collision|SetCollisionEnabled (Variables|Default|GetBox1) "NoCollision"))

(event Collision|EventActorBeginOverlap
  (params (OtherActor :type Actor%20Object%20Reference)))

(fn ConstructionScript)