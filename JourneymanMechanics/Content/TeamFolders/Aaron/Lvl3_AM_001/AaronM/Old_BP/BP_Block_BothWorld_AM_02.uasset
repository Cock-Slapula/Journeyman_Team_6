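; Block Blueprint that reacts to the player warping between a light and a dark world by changing its look.
; A WorldWarp event flips the MapStateDark flag and fires either LightMode or DarkMode.
; Both mode events only call SetMaterial on slot 0 of the static mesh, with no material specified in either call.
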(event Custom|World%20Warp
  ;[1 1 1] Checking which world the player is currently in and triggering the change
  (if (Variables|Default|GetMapState%20Dark)
    (CallFunction|LightMode)
    (Variables|Default|SetMapState%20Dark false)
    (else
      (CallFunction|DarkMode)
      (Variables|Default|SetMapState%20Dark true))))

(event Custom|Light%20Mode
  ;[0.8888 1 0.8712] Changes asset properties depending on which mode has been triggered
  (Rendering|Material|SetMaterial (Variables|Default|GetStaticMesh) 0 0))

(event Custom|Dark%20Mode
  ;[0.8888 1 0.8712] Changes asset properties depending on which mode has been triggered
  (Rendering|Material|SetMaterial (Variables|Default|GetStaticMesh) 0 0))

(fn ConstructionScript)