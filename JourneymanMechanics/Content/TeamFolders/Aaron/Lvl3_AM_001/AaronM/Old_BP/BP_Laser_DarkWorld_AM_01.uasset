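; Laser hazard for the dark/light world mechanic that kills Mario_Character on box overlap while in dark mode.
; WorldWarp toggles modes: dark shows the laser material and enables box collision, light swaps to glass and disables it.
; BeginPlay disables mesh and box collision and, if Rotation is set, one of four timelines lerps a full turn on roll or pitch in either direction, replaying via a delay.
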(event OnComponentBeginOverlap(Box)
  (params (OverlappedComponent :type Primitive%20Component%20Object%20Reference) (OtherActor :type Actor%20Object%20Reference) (OtherComp :type Primitive%20Component%20Object%20Reference) (OtherBodyIndex :type Integer) (bFromSweep :type Boolean) (SweepResult :type Hit%20Result%20Structure%20%28by%20ref%29))
  ;[1 1 1] Kills player on overlap
  (if (Variables|Default|GetCan%20Die)
    (bind _asmario_character (Utilities|Casting|CastToMario_Character OtherActor))
    (Default|IsDead _asmario_character)))

(event Custom|World%20Warp
  ;[1 1 1] Checking which world the player is currently in and triggering the change
  (if (Variables|Default|GetMapState%20Dark)
    (CallFunction|LightMode)
    (Variables|Default|SetMapState%20Dark false)
    (else
      (CallFunction|DarkMode)
      (Variables|Default|SetMapState%20Dark true))))

(event Custom|Light%20Mode
  ;[1 1 1] Changes asset properties depending on which mode has been triggered
  (Variables|Default|SetCan%20Die false)
  (Rendering|Material|SetMaterial (Variables|Default|GetStaticMesh) 0 "/Game/TeamFolders/Aaron/Lvl3_AM_001/AaronM/M_Glass.M_Glass")
  (Collision|SetCollisionEnabled (Variables|Default|GetBox) "NoCollision"))

(event Custom|Dark%20Mode
  ;[1 1 1] Changes asset properties depending on which mode has been triggered
  (Variables|Default|SetCan%20Die true)
  (Rendering|Material|SetMaterial (Variables|Default|GetStaticMesh) 0 "/Engine/VREditor/LaserPointer/LaserPointerMaterial.LaserPointerMaterial")
  (Collision|SetCollisionEnabled (Variables|Default|GetBox) "QueryAndPhysics"))

(event EventBeginPlay
  (bind _y (Variables|Default|GetY))
  (bind _y_2 (Variables|Default|GetY))
  (bind _y_3 (Variables|Default|GetY))
  (bind _y_4 (Variables|Default|GetY))
  (bind _staticmesh (Variables|Default|GetStaticMesh))
  (bind _relativerotation (Variables|/Script/Engine.SceneComponent|GetRelativeRotation _staticmesh))
  ;[1 1 1] Gets Coords, sets collision to none sets it so player can die
  (Variables|Default|SetRotation%20X (.roll _relativerotation))
  (Variables|Default|SetRotation%20Y (.pitch _relativerotation))
  (Variables|Default|SetRotation%20Z (.yaw _relativerotation))
  (Collision|SetCollisionEnabled (Variables|Default|GetStaticMesh) "NoCollision")
  (Variables|Default|SetCan%20Die true)
  (if (Variables|Default|GetRotation)
    ;[1 1 1] Laser Movement
    (if (Variables|Default|GetRotation%20Clockwise)
      (if (Variables|Default|GetY%20Rotation)
        (bind _newtrack_0 (Timeline|Timeline_1 Play)
          (:Update
            (Transformation|SetRelativeRotation (Variables|Default|GetStaticMesh) (Math|Rotator|Lerp(Rotator) (Math|Rotator|MakeRotator (Variables|Default|GetRotation%20X) _y_4 (Variables|Default|GetRotation%20Z)) (Math|Rotator|MakeRotator (Variables|Default|GetRotation%20X) (+ _y_4 -3.6e+02) (Variables|Default|GetRotation%20Z)) _newtrack_0) false false)
            (Utilities|FlowControl|Delay 5.0)
            (Timeline|Timeline_1 PlayFromStart)))
        (else
          (bind _newtrack_0_2 (Timeline|Timeline_0 Play)
            (:Update
              (Transformation|SetRelativeRotation (Variables|Default|GetStaticMesh) (Math|Rotator|Lerp(Rotator) (Math|Rotator|MakeRotator (Variables|Default|GetRotation%20X) _y_3 (Variables|Default|GetRotation%20Z)) (Math|Rotator|MakeRotator (+ (Variables|Default|GetRotation%20X) -3.6e+02) _y_3 (Variables|Default|GetRotation%20Z)) _newtrack_0_2) false false)
              (Utilities|FlowControl|Delay 5.0)
              (Timeline|Timeline_0 PlayFromStart)))))
      (elif (Variables|Default|GetY%20Rotation)
        (bind _newtrack_0_3 (Timeline|Timeline_3 Play)
          (:Update
            (Transformation|SetRelativeRotation (Variables|Default|GetStaticMesh) (Math|Rotator|Lerp(Rotator) (Math|Rotator|MakeRotator (Variables|Default|GetRotation%20X) _y (Variables|Default|GetRotation%20Z)) (Math|Rotator|MakeRotator (Variables|Default|GetRotation%20X) (+ _y 3.6e+02) (Variables|Default|GetRotation%20Z)) _newtrack_0_3) false false)
            (Utilities|FlowControl|Delay 5.0)
            (Timeline|Timeline_3 PlayFromStart)))
        (else
          (bind _newtrack_0_4 (Timeline|Timeline_2 Play)
            (:Update
              (Transformation|SetRelativeRotation (Variables|Default|GetStaticMesh) (Math|Rotator|Lerp(Rotator) (Math|Rotator|MakeRotator (Variables|Default|GetRotation%20X) _y_2 (Variables|Default|GetRotation%20Z)) (Math|Rotator|MakeRotator (+ (Variables|Default|GetRotation%20X) 3.6e+02) _y_2 (Variables|Default|GetRotation%20Z)) _newtrack_0_4) false false)
              (Utilities|FlowControl|Delay 5.0)
              (Timeline|Timeline_2 PlayFromStart))))))))

(fn ConstructionScript)