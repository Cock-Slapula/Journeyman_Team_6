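; Sliding surface for a light/dark world-switching level that makes Mario_Character slide while it overlaps the Box.
; WorldWarp flips MapStateDark and calls LightMode or DarkMode, which set the mesh material and toggle Box collision using the OnlyInDark and MirroredInDark flags.
; Box begin and end overlaps set and clear the character's IsSliding, and BeginPlay sets the initial material for dark-only surfaces.
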(event OnComponentBeginOverlap(Box)
  (params (OverlappedComponent :type Primitive%20Component%20Object%20Reference) (OtherActor :type Actor%20Object%20Reference) (OtherComp :type Primitive%20Component%20Object%20Reference) (OtherBodyIndex :type Integer) (bFromSweep :type Boolean) (SweepResult :type Hit%20Result%20Structure%20%28by%20ref%29))
  ;[1 1 1] Sets if player is sliding
  (bind _asmario_character (Utilities|Casting|CastToMario_Character OtherActor))
  (Variables|/Game/SideScrollerBP/Blueprints/Mario_Character.Mario_Character_C|SetIs%20Sliding _asmario_character true))

(event OnComponentEndOverlap(Box)
  (params (OverlappedComponent :type Primitive%20Component%20Object%20Reference) (OtherActor :type Actor%20Object%20Reference) (OtherComp :type Primitive%20Component%20Object%20Reference) (OtherBodyIndex :type Integer))
  ;[1 1 1] Sets if player is sliding
  (bind _asmario_character (Utilities|Casting|CastToMario_Character OtherActor))
  (Variables|/Game/SideScrollerBP/Blueprints/Mario_Character.Mario_Character_C|SetIs%20Sliding _asmario_character false))

(event Custom|World%20Warp
  ;[1 1 1] Checking which world the player is currently in and triggering the change
  (if (Variables|Default|GetMapState%20Dark)
    (CallFunction|LightMode)
    (Variables|Default|SetMapState%20Dark false)
    (else
      (CallFunction|DarkMode)
      (Variables|Default|SetMapState%20Dark true))))

(event Custom|Light%20Mode
  ;[1 1 1] Changes asset properties depending on which mode has been triggered
  (if (Variables|Default|GetOnly%20in%20Dark)
    (Variables|Default|SetMirrored%20in%20Dark true)
    (Rendering|Material|SetMaterial (Variables|Default|GetStaticMesh) 0 0)
    (Collision|SetCollisionEnabled (Variables|Default|GetBox) "NoCollision")
    (else
      (Rendering|Material|SetMaterial (Variables|Default|GetStaticMesh) 0 0)
      (Collision|SetCollisionEnabled (Variables|Default|GetBox) "QueryAndPhysics"))))

(event Custom|Dark%20Mode
  ;[1 1 1] Changes asset properties depending on which mode has been triggered
  (if (Variables|Default|GetMirrored%20in%20Dark)
    (Rendering|Material|SetMaterial (Variables|Default|GetStaticMesh) 0 0)
    (Collision|SetCollisionEnabled (Variables|Default|GetBox) "QueryAndPhysics")
    (else
      (Rendering|Material|SetMaterial (Variables|Default|GetStaticMesh) 0 0)
      (Collision|SetCollisionEnabled (Variables|Default|GetBox) "NoCollision"))))

(event EventBeginPlay
  (bind _staticmesh (Variables|Default|GetStaticMesh))
  (bind _relativelocation (Variables|/Script/Engine.SceneComponent|GetRelativeLocation _staticmesh))
  ;[1 1 1] Sets Material if Darkworld is icy
  (Variables|Default|SetY (.y _relativelocation))
  (Variables|Default|SetZ (.z _relativelocation))
  (if (Variables|Default|GetOnly%20in%20Dark)
    (Rendering|Material|SetMaterial (Variables|Default|GetStaticMesh) 0 0)))

(fn ConstructionScript)