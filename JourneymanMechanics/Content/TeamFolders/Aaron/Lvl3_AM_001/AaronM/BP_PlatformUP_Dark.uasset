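; Rising platform for a light/dark world-swap mechanic, solid in the Light state and a non-colliding glass ghost in the Dark state.
; On BeginPlay, a timeline lerps the mesh from its starting relative location toward a fixed raised point.
; HasSpawned and ChangeState share one state switch that sets visibility, collision and material.
; While Mario overlaps the DontSwap volume, switching to Light hides the mesh instead of making it solid.
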(event OnComponentBeginOverlap(Don'tSwap)
  (params (OverlappedComponent :type Primitive%20Component%20Object%20Reference) (OtherActor :type Actor%20Object%20Reference) (OtherComp :type Primitive%20Component%20Object%20Reference) (OtherBodyIndex :type Integer) (bFromSweep :type Boolean) (SweepResult :type Hit%20Result%20Structure%20%28by%20ref%29))
  ;[1 1 1] If Collided doesn't swap worlds
  (Utilities|Casting|CastToMario_Character OtherActor)
  (Variables|Default|SetDontSwap true))

(event OnComponentEndOverlap(Don'tSwap)
  (params (OverlappedComponent :type Primitive%20Component%20Object%20Reference) (OtherActor :type Actor%20Object%20Reference) (OtherComp :type Primitive%20Component%20Object%20Reference) (OtherBodyIndex :type Integer))
  ;[1 1 1] If Collided doesn't swap worlds
  (Utilities|Casting|CastToMario_Character OtherActor)
  (Variables|Default|SetDontSwap false))

(event Custom|HasSpawned
  (switch Utilities|FlowControl|Switch|SwitchonE_WorldSwitch (stale EventChangeState Current%20state)
    (:NewEnumerator0
      (Rendering|SetVisibility (Variables|Default|GetStaticMesh) true false)
      (Collision|SetCollisionEnabled (Variables|Default|GetStaticMesh) "NoCollision")
      (Rendering|Material|SetMaterial (Variables|Default|GetStaticMesh) 0 "/Game/TeamFolders/Aaron/Lvl3_AM_001/AaronM/M_Glass.M_Glass"))
    (:NewEnumerator1
      (if (Variables|Default|GetDontSwap)
        (Rendering|SetVisibility (Variables|Default|GetStaticMesh) false false)
        (else
          (Rendering|SetVisibility (Variables|Default|GetStaticMesh) true false)
          (Collision|SetCollisionEnabled (Variables|Default|GetStaticMesh) "QueryAndPhysics")
          (Rendering|Material|SetMaterial (Variables|Default|GetStaticMesh) 0 "/Game/SideScrollerBP/Materials/DarkWorld.DarkWorld"))))))

(event EventChangeState
  (params (Current%20state :type E_WorldSwitch%20Enum :default "NewEnumerator0"))
  (switch Utilities|FlowControl|Switch|SwitchonE_WorldSwitch Current%20state
    (:NewEnumerator0
      (Rendering|SetVisibility (Variables|Default|GetStaticMesh) true false)
      (Collision|SetCollisionEnabled (Variables|Default|GetStaticMesh) "NoCollision")
      (Rendering|Material|SetMaterial (Variables|Default|GetStaticMesh) 0 "/Game/TeamFolders/Aaron/Lvl3_AM_001/AaronM/M_Glass.M_Glass"))
    (:NewEnumerator1
      (if (Variables|Default|GetDontSwap)
        (Rendering|SetVisibility (Variables|Default|GetStaticMesh) false false)
        (else
          (Rendering|SetVisibility (Variables|Default|GetStaticMesh) true false)
          (Collision|SetCollisionEnabled (Variables|Default|GetStaticMesh) "QueryAndPhysics")
          (Rendering|Material|SetMaterial (Variables|Default|GetStaticMesh) 0 "/Game/SideScrollerBP/Materials/DarkWorld.DarkWorld"))))))

(event EventBeginPlay
  (Utilities|FlowControl|Sequence
    (:then_0
      (Variables|Default|SetStart_Location (Variables|/Script/Engine.SceneComponent|GetRelativeLocation (Variables|Default|GetStaticMesh))))
    (:then_1
      (bind _newtrack_0 (Timeline|Timeline_0 Play)
        (:Update
          (Transformation|SetRelativeLocation (Variables|Default|GetStaticMesh) (Math|Vector|Lerp(Vector) (Variables|Default|GetStart_Location) "0, 0,1000.000000" _newtrack_0) false false))))))

(fn ConstructionScript
  (|CallParentFunction))