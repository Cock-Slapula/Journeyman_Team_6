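; Conveyor belt block that reacts to Dark/Light world state changes and makes Mario slide while he overlaps its Box.
; Dark shows a non-colliding glass mesh; Light restores collision and the DarkWorld material.
; A DontSwap trigger flags Mario's overlap, so switching to Light then only hides the mesh instead of making it solid around him.
; Box overlaps toggle the character's IsSliding flag.
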(event OnComponentBeginOverlap(Don'tSwap)
  (params (OverlappedComponent :type Primitive%20Component%20Object%20Reference) (OtherActor :type Actor%20Object%20Reference) (OtherComp :type Primitive%20Component%20Object%20Reference) (OtherBodyIndex :type Integer) (bFromSweep :type Boolean) (SweepResult :type Hit%20Result%20Structure%20%28by%20ref%29))
  ;[1 1 1] If Collided doesn't swap worlds
  (Utilities|Casting|CastToMario_Character OtherActor)
  (Variables|Default|SetDontSwap true))

(event OnComponentEndOverlap(Don'tSwap)
  (params (OverlappedComponent :type Primitive%20Component%20Object%20Reference) (OtherActor :type Actor%20Object%20Reference) (OtherComp :type Primitive%20Component%20Object%20Reference) (OtherBodyIndex :type Integer))
  ;[1 1 1] If Collided doesn't swap worlds
  (Utilities|Casting|CastToMario_Character OtherActor)
  (Variables|Default|SetDontSwap false))

(event OnComponentBeginOverlap(Box)
  (params (OverlappedComponent :type Primitive%20Component%20Object%20Reference) (OtherActor :type Actor%20Object%20Reference) (OtherComp :type Primitive%20Component%20Object%20Reference) (OtherBodyIndex :type Integer) (bFromSweep :type Boolean) (SweepResult :type Hit%20Result%20Structure%20%28by%20ref%29))
  ;[1 1 1] Sets sliding
  (bind _asmario_character (Utilities|Casting|CastToMario_Character OtherActor))
  (Variables|/Game/SideScrollerBP/Blueprints/Mario_Character.Mario_Character_C|SetIs%20Sliding _asmario_character true))

(event OnComponentEndOverlap(Box)
  (params (OverlappedComponent :type Primitive%20Component%20Object%20Reference) (OtherActor :type Actor%20Object%20Reference) (OtherComp :type Primitive%20Component%20Object%20Reference) (OtherBodyIndex :type Integer))
  ;[1 1 1] Sets sliding
  (bind _asmario_character (Utilities|Casting|CastToMario_Character OtherActor))
  (Variables|/Game/SideScrollerBP/Blueprints/Mario_Character.Mario_Character_C|SetIs%20Sliding _asmario_character false))

(event EventChangeState
  (params (Current%20state :type E_WorldSwitch%20Enum :default "NewEnumerator0"))
  (switch Utilities|FlowControl|Switch|SwitchonE_WorldSwitch Current%20state
    (:NewEnumerator0
      (Rendering|SetVisibility (Variables|Default|GetStaticMesh) true false)
      (Collision|SetCollisionEnabled (Variables|Default|GetStaticMesh) "NoCollision")
      (Rendering|Material|SetMaterial (Variables|Default|GetStaticMesh) 0 "/Game/TeamFolders/Aaron/Lvl3_AM_001/AaronM/M_Glass.M_Glass"))
    (:NewEnumerator1
      (if (Variables|Default|GetDontSwap)
        (Rendering|SetVisibility (Variables|Default|GetStaticMesh) false false)
        (else
          (Rendering|SetVisibility (Variables|Default|GetStaticMesh) true false)
          (Collision|SetCollisionEnabled (Variables|Default|GetStaticMesh) "QueryAndPhysics")
          (Rendering|Material|SetMaterial (Variables|Default|GetStaticMesh) 0 "/Game/SideScrollerBP/Materials/DarkWorld.DarkWorld"))))))

(fn ConstructionScript
  (|CallParentFunction))