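; Moving platform for a Light/Dark world-swap mechanic: solid in Dark, non-colliding glass in Light.
; If Mario overlaps the DontSwap volume, switching to Dark hides the mesh and leaves collision unchanged.
; Box overlap drives a timeline lerp to EndLocation with delayed reversal, or, in Drop mode, DropBox turns it red and lowers it after a delay.
; Leaving DropBox later spawns a Bp_Block_Dark_Moving, not this class, at StartLocation's relative coordinates.
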(event OnComponentBeginOverlap(Don'tSwap)
  (params (OverlappedComponent :type Primitive%20Component%20Object%20Reference) (OtherActor :type Actor%20Object%20Reference) (OtherComp :type Primitive%20Component%20Object%20Reference) (OtherBodyIndex :type Integer) (bFromSweep :type Boolean) (SweepResult :type Hit%20Result%20Structure%20%28by%20ref%29))
  ;[1 1 1] If Collided doesn't swap worlds
  (Utilities|Casting|CastToMario_Character OtherActor)
  (Variables|Default|SetDon'tSwap true))

(event OnComponentEndOverlap(Don'tSwap)
  (params (OverlappedComponent :type Primitive%20Component%20Object%20Reference) (OtherActor :type Actor%20Object%20Reference) (OtherComp :type Primitive%20Component%20Object%20Reference) (OtherBodyIndex :type Integer))
  ;[1 1 1] If Collided doesn't swap worlds
  (Utilities|Casting|CastToMario_Character OtherActor)
  (Variables|Default|SetDon'tSwap false))

(event OnComponentBeginOverlap(Box)
  (params (OverlappedComponent :type Primitive%20Component%20Object%20Reference) (OtherActor :type Actor%20Object%20Reference) (OtherComp :type Primitive%20Component%20Object%20Reference) (OtherBodyIndex :type Integer) (bFromSweep :type Boolean) (SweepResult :type Hit%20Result%20Structure%20%28by%20ref%29))
  ;[1 1 1] Movement
  (Utilities|Casting|CastToMario_Character OtherActor)
  (if (not (Variables|Default|GetDrop))
    (bind _newtrack_0 (Timeline|Timeline_1 Play)
      (:Update
        (Transformation|SetRelativeLocation (Variables|Default|GetStaticMesh) (Math|Vector|Lerp(Vector) (Variables|Default|GetStartLocation) (Variables|Default|GetEndLocation) _newtrack_0) false false)
        (Utilities|FlowControl|Delay 1e+01)
        (Timeline|Timeline_1 Reverse)))))

(event OnComponentBeginOverlap(DropBox)
  (params (OverlappedComponent :type Primitive%20Component%20Object%20Reference) (OtherActor :type Actor%20Object%20Reference) (OtherComp :type Primitive%20Component%20Object%20Reference) (OtherBodyIndex :type Integer) (bFromSweep :type Boolean) (SweepResult :type Hit%20Result%20Structure%20%28by%20ref%29))
  ;[1 1 1] Drop
  (Utilities|Casting|CastToMario_Character OtherActor)
  (if (Variables|Default|GetDrop)
    (Variables|Default|SetActivated true)
    (Rendering|Material|SetMaterial (Variables|Default|GetStaticMesh) 0 "/Game/TeamFolders/Martin/Materials/M_Red_Dark.M_Red_Dark")
    (Utilities|FlowControl|Delay 2.0)
    (bind _newtrack_0 (Timeline|Timeline_0 Play)
      (:Update
        (Transformation|SetRelativeLocation (Variables|Default|GetStaticMesh) (Math|Vector|Lerp(Vector) (Variables|Default|GetStartLocation) (Variables|Default|GetDropLocation) _newtrack_0) false false)
        (Utilities|FlowControl|Delay 5.0)))))

(event OnComponentEndOverlap(DropBox)
  (params (OverlappedComponent :type Primitive%20Component%20Object%20Reference) (OtherActor :type Actor%20Object%20Reference) (OtherComp :type Primitive%20Component%20Object%20Reference) (OtherBodyIndex :type Integer))
  ;[1 1 1] If Dropping Respawn
  (Utilities|Casting|CastToMario_Character OtherActor)
  (if (Variables|Default|GetDrop)
    (Utilities|FlowControl|Delay 5.5)
    (Game|SpawnActorfromClass "/Game/TeamFolders/Aaron/Lvl3_AM_001/AaronM/Bp_Block_Dark_Moving.Bp_Block_Dark_Moving_C" (Math|Transform|MakeTransform (Variables|Default|GetStartLocation) "0, 0, 0" "1,1,1") "Undefined" 0 0)))

(event EventBeginPlay
  ;[1 1 1] Gets Coords
  (Variables|Default|SetStartLocation (Variables|/Script/Engine.SceneComponent|GetRelativeLocation (Variables|Default|GetStaticMesh)))
  (Variables|Default|SetEndLocation (Variables|/Script/Engine.SceneComponent|GetRelativeLocation (Variables|Default|GetEnd%20Location)))
  (Variables|Default|SetDropLocation (Variables|/Script/Engine.SceneComponent|GetRelativeLocation (Variables|Default|GetDrop%20Location))))

(event EventChangeState
  (params (Current%20state :type E_WorldSwitch%20Enum :default "NewEnumerator0"))
  (switch Utilities|FlowControl|Switch|SwitchonE_WorldSwitch Current%20state
    (:NewEnumerator0
      (if (Variables|Default|GetDon'tSwap)
        (Rendering|SetVisibility (Variables|Default|GetStaticMesh) false false)
        (elif (Variables|Default|GetActivated)
          (Rendering|SetVisibility (Variables|Default|GetStaticMesh) true false)
          (Collision|SetCollisionEnabled (Variables|Default|GetStaticMesh) "QueryAndPhysics")
          (Rendering|Material|SetMaterial (Variables|Default|GetStaticMesh) 0 "/Game/TeamFolders/Martin/Materials/M_Red_Dark.M_Red_Dark")
          (else
            (Rendering|SetVisibility (Variables|Default|GetStaticMesh) true false)
            (Collision|SetCollisionEnabled (Variables|Default|GetStaticMesh) "QueryAndPhysics")
            (Rendering|Material|SetMaterial (Variables|Default|GetStaticMesh) 0 "/Game/TeamFolders/Martin/Materials/M_White.M_White")))))
    (:NewEnumerator1
      (Rendering|SetVisibility (Variables|Default|GetStaticMesh) true false)
      (Collision|SetCollisionEnabled (Variables|Default|GetStaticMesh) "NoCollision")
      (Rendering|Material|SetMaterial (Variables|Default|GetStaticMesh) 0 "/Game/TeamFolders/Aaron/Lvl3_AM_001/AaronM/M_Glass.M_Glass"))))

(fn ConstructionScript
  (|CallParentFunction))