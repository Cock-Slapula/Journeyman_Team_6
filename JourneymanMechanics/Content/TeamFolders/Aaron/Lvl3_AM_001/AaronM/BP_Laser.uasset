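; BP_Laser is a laser hazard that can rotate and switches with a Dark/Light state.
; BeginPlay optionally starts one of four timelines, chosen by direction and axis, lerping the mesh a full turn in roll or pitch and restarting after a delay.
; ChangeState shows glass with collision off in Dark, and laser material with the hit box enabled in Light.
; Mario_Character overlapping the box only prints "DEAD".
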(event OnComponentBeginOverlap(Box)
  (params (OverlappedComponent :type Primitive%20Component%20Object%20Reference) (OtherActor :type Actor%20Object%20Reference) (OtherComp :type Primitive%20Component%20Object%20Reference) (OtherBodyIndex :type Integer) (bFromSweep :type Boolean) (SweepResult :type Hit%20Result%20Structure%20%28by%20ref%29))
  ;[1 1 1] Kills Player
  (Utilities|Casting|CastToMario_Character OtherActor)
  (Development|PrintString "DEAD"))

(event EventBeginPlay
  (bind _staticmesh (Variables|Default|GetStaticMesh))
  (bind _relativerotation (Variables|/Script/Engine.SceneComponent|GetRelativeRotation _staticmesh))
  ;[1 1 1] Gets Coords
  (Variables|Default|SetRotaion%20X (.roll _relativerotation))
  (Variables|Default|SetRotation%20Y (.pitch _relativerotation))
  (Variables|Default|SetRotation%20Z (.yaw _relativerotation))
  (if (Variables|Default|GetRotation)
    ;[1 1 1] Movement
    (if (Variables|Default|GetRotate%20Clockwise)
      (if (Variables|Default|GetRotate%20on%20Y%20axis)
        (bind _newtrack_0 (Timeline|Timeline_2 Play)
          (:Update
            (Transformation|SetRelativeRotation (Variables|Default|GetStaticMesh) (Math|Rotator|Lerp(Rotator) (Math|Rotator|MakeRotator (Variables|Default|GetRotaion%20X) (Variables|Default|GetRotation%20Y) (Variables|Default|GetRotation%20Z)) (Math|Rotator|MakeRotator (Variables|Default|GetRotaion%20X) (+ (Variables|Default|GetRotation%20Y) -3.6e+02) (Variables|Default|GetRotation%20Z)) _newtrack_0) false false)
            (Utilities|FlowControl|Delay 5.0)
            (Timeline|Timeline_2 PlayFromStart)))
        (else
          (bind _newtrack_0_2 (Timeline|Timeline_3 Play)
            (:Update
              (Transformation|SetRelativeRotation (Variables|Default|GetStaticMesh) (Math|Rotator|Lerp(Rotator) (Math|Rotator|MakeRotator (Variables|Default|GetRotaion%20X) (Variables|Default|GetRotation%20Y) (Variables|Default|GetRotation%20Z)) (Math|Rotator|MakeRotator (+ (Variables|Default|GetRotaion%20X) -3.6e+02) (Variables|Default|GetRotation%20Y) (Variables|Default|GetRotation%20Z)) _newtrack_0_2) false false)
              (Utilities|FlowControl|Delay 5.0)
              (Timeline|Timeline_3 PlayFromStart)))))
      (elif (Variables|Default|GetRotate%20on%20Y%20axis)
        (bind _newtrack_0_3 (Timeline|Timeline_0 Play)
          (:Update
            (Transformation|SetRelativeRotation (Variables|Default|GetStaticMesh) (Math|Rotator|Lerp(Rotator) (Math|Rotator|MakeRotator (Variables|Default|GetRotaion%20X) (Variables|Default|GetRotation%20Y) (Variables|Default|GetRotation%20Z)) (Math|Rotator|MakeRotator (Variables|Default|GetRotaion%20X) (+ (Variables|Default|GetRotation%20Y) 3.6e+02) (Variables|Default|GetRotation%20Z)) _newtrack_0_3) false false)
            (Utilities|FlowControl|Delay 5.0)
            (Timeline|Timeline_0 PlayFromStart)))
        (else
          (bind _newtrack_0_4 (Timeline|Timeline_1 Play)
            (:Update
              (Transformation|SetRelativeRotation (Variables|Default|GetStaticMesh) (Math|Rotator|Lerp(Rotator) (Math|Rotator|MakeRotator (Variables|Default|GetRotaion%20X) (Variables|Default|GetRotation%20Y) (Variables|Default|GetRotation%20Z)) (Math|Rotator|MakeRotator (+ (Variables|Default|GetRotaion%20X) 3.6e+02) (Variables|Default|GetRotation%20Y) (Variables|Default|GetRotation%20Z)) _newtrack_0_4) false false)
              (Utilities|FlowControl|Delay 5.0)
              (Timeline|Timeline_1 PlayFromStart))))))))

(event EventChangeState
  (params (Current%20state :type E_WorldSwitch%20Enum :default "NewEnumerator0"))
  (switch Utilities|FlowControl|Switch|SwitchonE_WorldSwitch Current%20state
    (:NewEnumerator0
      (Rendering|SetVisibility (Variables|Default|GetStaticMesh) true false)
      (Collision|SetCollisionEnabled (Variables|Default|GetStaticMesh) "NoCollision")
      (Rendering|Material|SetMaterial (Variables|Default|GetStaticMesh) 0 "/Game/TeamFolders/Aaron/Lvl3_AM_001/AaronM/M_Glass.M_Glass"))
    (:NewEnumerator1
      (Rendering|SetVisibility (Variables|Default|GetStaticMesh) true false)
      (Collision|SetCollisionEnabled (Variables|Default|GetStaticMesh) "NoCollision")
      (Rendering|Material|SetMaterial (Variables|Default|GetStaticMesh) 0 "/Engine/VREditor/LaserPointer/LaserPointerMaterial.LaserPointerMaterial")
      (Collision|SetCollisionEnabled (Variables|Default|GetBox) "QueryAndPhysics"))))

(fn ConstructionScript
  (|CallParentFunction))