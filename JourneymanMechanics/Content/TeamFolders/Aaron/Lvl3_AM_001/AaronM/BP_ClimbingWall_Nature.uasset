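; Climbing wall that toggles between solid and ghosted as the game switches between Dark and Light worlds.
; ChangeState uses SetDarkWorld to pick the world where mesh, climbing collision and arrow lose collision and the mesh turns glass; the other world restores them.
; A Box overlap with Mario_Character sets DontSwap, so a switch that would restore the wall only hides the mesh, leaving collision unchanged.
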(event OnComponentBeginOverlap(Box)
  (params (OverlappedComponent :type Primitive%20Component%20Object%20Reference) (OtherActor :type Actor%20Object%20Reference) (OtherComp :type Primitive%20Component%20Object%20Reference) (OtherBodyIndex :type Integer) (bFromSweep :type Boolean) (SweepResult :type Hit%20Result%20Structure%20%28by%20ref%29))
  ;[1 1 1] If Collided doesn't swap worlds
  (Utilities|Casting|CastToMario_Character OtherActor)
  (Variables|Default|SetDontSwap true))

(event OnComponentEndOverlap(Box)
  (params (OverlappedComponent :type Primitive%20Component%20Object%20Reference) (OtherActor :type Actor%20Object%20Reference) (OtherComp :type Primitive%20Component%20Object%20Reference) (OtherBodyIndex :type Integer))
  ;[1 1 1] If Collided doesn't swap worlds
  (Utilities|Casting|CastToMario_Character OtherActor)
  (Variables|Default|SetDontSwap false))

(event EventChangeState
  (params (Current%20state :type E_WorldSwitch%20Enum :default "NewEnumerator0"))
  (bind _setdarkworld (Variables|Default|GetSetDarkWorld))
  (switch Utilities|FlowControl|Switch|SwitchonE_WorldSwitch Current%20state
    (:NewEnumerator0
      (if _setdarkworld
        (Rendering|SetVisibility (Variables|Default|GetStaticMesh) true false)
        (Collision|SetCollisionEnabled (Variables|Default|GetStaticMesh) "NoCollision")
        (Rendering|Material|SetMaterial (Variables|Default|GetStaticMesh) 0 "/Game/TeamFolders/Aaron/Lvl3_AM_001/AaronM/M_Glass.M_Glass")
        (Collision|SetCollisionEnabled (Variables|Default|GetClimbing%20Collision) "NoCollision")
        (Variables|Default|SetDarkWorld true)
        (elif (Variables|Default|GetDontSwap)
          (Rendering|SetVisibility (Variables|Default|GetStaticMesh) false false)
          (else
            (Rendering|SetVisibility (Variables|Default|GetStaticMesh) true false)
            (Collision|SetCollisionEnabled (Variables|Default|GetStaticMesh) "QueryAndPhysics")
            (Rendering|Material|SetMaterial (Variables|Default|GetStaticMesh) 0 "/Game/TeamFolders/Martin/Materials/M_White.M_White")
            (Collision|SetCollisionEnabled (Variables|Default|GetClimbing%20Collision) "QueryOnly")
            (Variables|Default|SetDarkWorld false)))))
    (:NewEnumerator1
      (if _setdarkworld
        (if (Variables|Default|GetDontSwap)
          (Rendering|SetVisibility (Variables|Default|GetStaticMesh) false false)
          (else
            (Rendering|SetVisibility (Variables|Default|GetStaticMesh) true false)
            (Collision|SetCollisionEnabled (Variables|Default|GetStaticMesh) "QueryAndPhysics")
            (Rendering|Material|SetMaterial (Variables|Default|GetStaticMesh) 0 "/Game/SideScrollerBP/Materials/DarkWorld.DarkWorld")
            (Collision|SetCollisionEnabled (Variables|Default|GetClimbing%20Collision) "QueryOnly")
            (Variables|Default|SetDarkWorld false)))
        (else
          (Rendering|SetVisibility (Variables|Default|GetStaticMesh) true false)
          (Collision|SetCollisionEnabled (Variables|Default|GetStaticMesh) "NoCollision")
          (Rendering|Material|SetMaterial (Variables|Default|GetStaticMesh) 0 "/Game/TeamFolders/Aaron/Lvl3_AM_001/AaronM/M_Glass.M_Glass")
          (Collision|SetCollisionEnabled (Variables|Default|GetClimbing%20Collision) "NoCollision")
          (Variables|Default|SetDarkWorld true))))))

(fn ConstructionScript
  (|CallParentFunction))