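; BP_Pickups is an item pickup whose mesh is chosen by index in the construction script.
; When Mario_Character overlaps its box, it records the item on the character, updates the W_Items HUD widget and destroys itself.
; If an item is already held, it spawns that item as a new pickup at the player.
; Swapped-out pickups show a non-interactive material for a few seconds before becoming collectable.
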(event OnComponentBeginOverlap(Box)
  (params (OverlappedComponent :type Primitive%20Component%20Object%20Reference) (OtherActor :type Actor%20Object%20Reference) (OtherComp :type Primitive%20Component%20Object%20Reference) (OtherBodyIndex :type Integer) (bFromSweep :type Boolean) (SweepResult :type Hit%20Result%20Structure%20%28by%20ref%29))
  ;[1 1 1] Sets HUD Icon, Deletes Actor Picked Up
  (bind _asmario_character (Utilities|Casting|CastToMario_Character OtherActor))
  (if (Variables|Default|GetInteractable)
    (if (Variables|/Game/SideScrollerBP/Blueprints/Mario_Character.Mario_Character_C|GetItemInHUD? _asmario_character)
      (CallFunction|Swap)
      (Variables|/Game/SideScrollerBP/Blueprints/Mario_Character.Mario_Character_C|SetItemHeld _asmario_character (Variables|Default|GetMeshIndex))
      (else
        (CallFunction|PickUp)))))

(event Custom|Pick%20Up
  (bind _meshindex (Variables|Default|GetMeshIndex))
  ;[1 1 1] Pick Up
  (Variables|/Game/SideScrollerBP/Blueprints/Mario_Character.Mario_Character_C|SetItemHeld (stale OnComponentBeginOverlap(Box) _asmario_character) _meshindex)
  (Variables|/Game/SideScrollerBP/Blueprints/Mario_Character.Mario_Character_C|SetItemInHUD? (stale OnComponentBeginOverlap(Box) _asmario_character) true)
  (bind _foundwidgets (Widget|GetAllWidgetsOfClass "/Game/TeamFolders/Rachel/RC-Inventory/Widgets/W_Items.W_Items_C" true))
  (Variables|/Game/TeamFolders/Rachel/RC-Inventory/Widgets/W_Items.W_Items_C|SetWhichItem (Utilities|Array|Get(acopy) _foundwidgets) _meshindex)
  (Default|ItemSelected (Utilities|Array|Get(acopy) _foundwidgets))
  (Actor|DestroyActor))

(event Custom|Swap
  ;[1 1 1] Swapping Item
  (Actor|DestroyActor)
  (Game|SpawnActorfromClass "BP_Pickups_C" (Math|Conversions|ToTransform(Vector) (Transformation|GetSocketLocation (Variables|/Script/Engine.Character|GetMesh (Game|GetPlayerCharacter 0)) "None")) "Undefined" 0 false (Variables|/Game/SideScrollerBP/Blueprints/Mario_Character.Mario_Character_C|GetItemHeld (stale OnComponentBeginOverlap(Box) _asmario_character)) true 0)
  (bind _foundwidgets (Widget|GetAllWidgetsOfClass "/Game/TeamFolders/Rachel/RC-Inventory/Widgets/W_Items.W_Items_C" true))
  (Variables|/Game/TeamFolders/Rachel/RC-Inventory/Widgets/W_Items.W_Items_C|SetWhichItem (Utilities|Array|Get(acopy) _foundwidgets) (Variables|Default|GetMeshIndex))
  (Default|ItemSelected (Utilities|Array|Get(acopy) _foundwidgets)))

(event Custom|Interactive%20Material
  ;[1 1 1] Flashing material for dropped items
  (Rendering|Material|SetMaterial (Variables|Default|GetPickupMesh) 0 (Variables|Default|GetInteractive%20Materal)))

(event Custom|Non-Ineractive%20Material
  ;[1 1 1] Flashing material for dropped items
  (Rendering|Material|SetMaterial (Variables|Default|GetPickupMesh) 0 "/Game/TeamFolders/Rachel/RC-Inventory/PickupMaterials/M_Non-Interactive.M_Non-Interactive"))

(event EventBeginPlay
  ;[1 1 1] Makes Swapped Items Non-Interactable For 3 Secs After Spawning
  (Variables|Default|SetInteractive%20Materal (Rendering|Material|GetMaterial (Variables|Default|GetPickupMesh) 0))
  (if (Variables|Default|GetSpawned)
    (CallFunction|Non-IneractiveMaterial)
    (Utilities|FlowControl|Delay 3.0)
    (Variables|Default|SetInteractable true)
    (CallFunction|InteractiveMaterial)))

(fn ConstructionScript
  (Components|StaticMesh|SetStaticMesh (Variables|Default|GetPickupMesh) (Utilities|Array|Get(acopy) (Variables|Default|GetMesh) (Variables|Default|GetMeshIndex))))