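; BP_Random_Box is an item box that gives an overlapping Mario_Character a random pickup.
; If an item is already held and no roll is running, it also spawns that item as a BP_Pickups at player 0's mesh.
; ChooseRandom removes the box's collision and mesh, shows a placeholder selection in W_Items, and waits briefly.
; It then picks an item index from an editable range, updates the character and HUD, and destroys itself.
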(event OnComponentBeginOverlap(Collision)
  (params (OverlappedComponent :type Primitive%20Component%20Object%20Reference) (OtherActor :type Actor%20Object%20Reference) (OtherComp :type Primitive%20Component%20Object%20Reference) (OtherBodyIndex :type Integer) (bFromSweep :type Boolean) (SweepResult :type Hit%20Result%20Structure%20%28by%20ref%29))
  ;[1 1 1] Check Inventory
  (bind _asmario_character (Utilities|Casting|CastToMario_Character OtherActor))
  (if (Variables|/Game/SideScrollerBP/Blueprints/Mario_Character.Mario_Character_C|GetItemInHUD? _asmario_character)
    (if (not (Variables|/Game/SideScrollerBP/Blueprints/Mario_Character.Mario_Character_C|GetChoosingItem? _asmario_character))
      ;[1 1 1] Drop Held Item
      (CallFunction|ChooseRandom)
      (Game|SpawnActorfromClass "/Game/TeamFolders/Rachel/RC-Inventory/BP/BP_Pickups.BP_Pickups_C" (Math|Conversions|ToTransform(Vector) (Transformation|GetSocketLocation (Variables|/Script/Engine.Character|GetMesh (Game|GetPlayerCharacter 0)) "None")) "Undefined" 0 false (Variables|/Game/SideScrollerBP/Blueprints/Mario_Character.Mario_Character_C|GetItemHeld _asmario_character) true 0))
    (else
      (CallFunction|ChooseRandom))))

(event Custom|ChooseRandom
  ;[1 1 1] Choose Random Pickup
  (Variables|/Game/SideScrollerBP/Blueprints/Mario_Character.Mario_Character_C|SetChoosingItem? (stale OnComponentBeginOverlap(Collision) _asmario_character) true)
  (Variables|/Game/SideScrollerBP/Blueprints/Mario_Character.Mario_Character_C|SetItemInHUD? (stale OnComponentBeginOverlap(Collision) _asmario_character) true)
  (Components|DestroyComponent (Variables|Default|GetCollision))
  (bind _foundwidgets (Widget|GetAllWidgetsOfClass "/Game/TeamFolders/Rachel/RC-Inventory/Widgets/W_Items.W_Items_C" true))
  (Variables|/Game/TeamFolders/Rachel/RC-Inventory/Widgets/W_Items.W_Items_C|SetWhichItem (Utilities|Array|Get(acopy) _foundwidgets) 4)
  (Default|ItemSelected (Utilities|Array|Get(acopy) _foundwidgets))
  (Utilities|FlowControl|Delay 3.0)
  (bind _output_get (Variables|/Game/SideScrollerBP/Blueprints/Mario_Character.Mario_Character_C|SetItemHeld (stale OnComponentBeginOverlap(Collision) _asmario_character) (Math|Random|RandomIntegerinRange (Variables|Default|GetPickup%20Range%201) (Variables|Default|GetPickup%20Range%202))))
  (Variables|/Game/TeamFolders/Rachel/RC-Inventory/Widgets/W_Items.W_Items_C|SetWhichItem (Utilities|Array|Get(acopy) _foundwidgets) _output_get)
  (Default|ItemSelected (Utilities|Array|Get(acopy) _foundwidgets))
  (Variables|/Game/SideScrollerBP/Blueprints/Mario_Character.Mario_Character_C|SetChoosingItem? (stale OnComponentBeginOverlap(Collision) _asmario_character) false)
  (Actor|DestroyActor))

(fn ConstructionScript)